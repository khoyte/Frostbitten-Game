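; ShovelSnow_BP is a shoveled snow pile that can grow, shrink and be destroyed, reacting when a Frost Stalker hits it.
; A hit sets StopMoving, waits longer for bigger piles, clears the flag, then runs staggered SubtractingSnow calls.
; AddingSnow scales the pile up to MaxSize, costing player RunStamina; SubtractingSnow scales it down, destroying it at minimum size.
; Logic updating Shoveling_PC's pile count is disconnected.
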(event `self.ReceiveHit`
  (params (MyComp :type "PrimitiveComponent Object Reference") (Other :type "Actor Object Reference") (OtherComp :type "PrimitiveComponent Object Reference") (bSelfMoved :type Boolean) (HitLocation :type "Vector Structure") (HitNormal :type "Vector Structure") (NormalImpulse :type "Vector Structure") (Hit :type "HitResult Structure (by ref)"))
  (bind _total_size (`self.total size`))
  ;[1 1 1] Frost Stalker Collide and then destroy snow pile.
  (cast `/Game/Blueprints/Enemy/Alex/Frost_Stalker_BP` Other)
  (set `self.StopMoving` true)
  (if (== _total_size 1)
    (`KismetSystemLibrary.Delay` 3.0)
    (set `self.StopMoving` false)
    (`self.Subtracting Snow`)
    (elif (== _total_size 2)
      (`KismetSystemLibrary.Delay` 5.0)
      (set `self.StopMoving` false)
      (`self.Subtracting Snow`)
      (`KismetSystemLibrary.Delay` 0.5)
      (`self.Subtracting Snow`)
      (else
        (`KismetSystemLibrary.Delay` 7.0)
        (set `self.StopMoving` false)
        (`self.Subtracting Snow`)
        (`KismetSystemLibrary.Delay` 0.5)
        (`self.Subtracting Snow`)
        (`KismetSystemLibrary.Delay` 0.5)
        (`self.Subtracting Snow`)
        (`KismetSystemLibrary.Delay` 0.5)
        (`self.Subtracting Snow`)
        (`KismetSystemLibrary.Delay` 0.5)
        (`self.Subtracting Snow`)))))

(event `self.ReceiveBeginPlay`)

(event `self.ReceiveDestroyed`)

(fn `Adding Snow`
  (if (< (`self.total size`) (`self.Max Size`))
    (`self.SetActorScale3D` (* (`self.GetActorScale3D`) 1.2))
    (set `self.total size` (+ (`self.total size`) 1))
    (set `self.Add Snow` false)
    (bind _asplayer (cast `/Game/Player_Content/Player` (`GameplayStatics.GetPlayerCharacter` 0)))
    (set `/Game/Player_Content/Player.RunStamina` (- (`/Game/Player_Content/Player.RunStamina` _asplayer) 1.0) _asplayer)
    (else
      (set `self.Add Snow` false))))

(fn `Subtracting Snow`
  (if (> (`self.total size`) (`self.Min Size`))
    (`self.SetActorScale3D` (/ (`self.GetActorScale3D`) 1.2))
    (set `self.total size` (- (`self.total size`) (`self.Min Size`)))
    (set `self.Substract Snow` false)
    (else
      (`self.K2_DestroyActor`))))

(fn `UserConstructionScript`)