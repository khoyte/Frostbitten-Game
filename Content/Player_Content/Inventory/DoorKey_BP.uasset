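; DoorKey_BP is a door key pickup that the player collects with Interact while inside its sphere.
; Sphere overlap shows a press-E prompt and opens a Gate that lets Interact through; leaving removes the prompt and closes it.
; Pickup adds the item to inventory, adds an objective, sets HasDoorKey on the game instance, plays sounds and destroys the actor.
; UseItem only plays a dialogue or sound cue.
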(event `UseItem`
  (`GameplayStatics.PlaySound2D` "/Game/Audio/Voice/JoshsStation/Dial_JS10.Dial_JS10" 1.0 1.0 0.0 null null))

(event `/Game/Player_Content/Interaction_Mechanic.Interact`
  (`/Engine/EditorBlueprintResources/StandardMacros.Gate` true :!label _label
    (:`Exit`
      (bind _asplayer (cast `/Game/Player_Content/Player` (`GameplayStatics.GetPlayerCharacter` 0)))
      (`/Game/Player_Content/Inventory/Inventory_WU.AddToInventory` (`/Game/Player_Content/Player.Inventory_Widget` _asplayer) (`self.ItemInfo`))
      (`GameplayStatics.PlaySound2D` "/Game/Audio/SFX/SFX_GrabSound.SFX_GrabSound" 1.0 1.0 0.0 null null)
      (`/Game/Player_Content/Player.AddObjective` _asplayer (`self.Objective`))
      (bind _asfrostbitten_game_inst_bp (cast `/Game/Blueprints/FrostbittenGameInst_BP` (`GameplayStatics.GetGameInstance`)))
      (set `/Game/Blueprints/FrostbittenGameInst_BP.hasDoorKey?` true _asfrostbitten_game_inst_bp)
      (`GameplayStatics.PlaySound2D` "/Game/Audio/Voice/JoshsStation/Dial_JS10.Dial_JS10" 1.0 1.0 0.0 null null)
      (`self.K2_DestroyActor`))))

(event `self.Sphere.OnComponentBeginOverlap`
  (params (OverlappedComponent :type "PrimitiveComponent Object Reference") (OtherActor :type "Actor Object Reference") (OtherComp :type "PrimitiveComponent Object Reference") (OtherBodyIndex :type Integer) (bFromSweep :type Boolean) (SweepResult :type "HitResult Structure (by ref)"))
  (cast `/Game/Player_Content/Player` OtherActor)
  (`/Engine/EditorBlueprintResources/StandardMacros.DoOnce` false :!label _label_2
    (:`Completed`
      (bind _returnvalue (`|CreateWidget` "/Game/Blueprints/Widgets/PressEtoPickUp_BP.PressEtoPickUp_BP_C"))
      (bind _output_get (set `self.PressE` _returnvalue))
      (`UserWidget.AddToViewport` _output_get 0)
      (goto _label :!via `Open`))))

(event `self.Sphere.OnComponentEndOverlap`
  (params (OverlappedComponent :type "PrimitiveComponent Object Reference") (OtherActor :type "Actor Object Reference") (OtherComp :type "PrimitiveComponent Object Reference") (OtherBodyIndex :type Integer))
  (bind _presse (`self.PressE`))
  (cast `/Game/Player_Content/Player` OtherActor)
  (`/Engine/EditorBlueprintResources/StandardMacros.IsValid` _presse
    (:`Is Valid`
      (`Widget.RemoveFromParent` _presse)
      (`|ExecutionSequence`
        (:`then_0`
          (goto _label_2 :!via `Reset`))
        (:`then_1`
          (goto _label :!via `Close`))))))

(fn `UserConstructionScript`)