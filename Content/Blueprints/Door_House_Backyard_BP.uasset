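; House door to the Backyard level, which stays locked until the game instance reports all toys collected.
; A box overlap enables input for the player; interacting while locked plays a locked-door sound.
; When unlocked, a FlipFlop plays or reverses a timeline that yaws the Arrow component.
; The timeline's update pin also runs a short delay, then saves player data and opens Backyard, so the level can change mid-swing.
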(event `self.ReceiveBeginPlay`
  (bind _asfrostbitten_game_inst_bp (cast `/Game/Blueprints/FrostbittenGameInst_BP` (`GameplayStatics.GetGameInstance`)))
  (set `self.GameInstance` _asfrostbitten_game_inst_bp))

(event `InputAction|Interact`
  (params (Key :type "Key Structure"))
  (:`Pressed`
    (if (`/Game/Blueprints/FrostbittenGameInst_BP.AllToysCollected?` (`self.GameInstance`))
      (`/Engine/EditorBlueprintResources/StandardMacros.FlipFlop`
        (:`A`
          (bind (_direction _door_track) (`Timeline|Door` :!label _label)
            (:`Update`
              (`SceneComponent.K2_SetRelativeRotation` (`self.Arrow`) (`KismetMathLibrary.MakeRotator` 0.0 0.0 (* _door_track (`self.Angle`))) false false)
              (`KismetSystemLibrary.Delay` 0.15)
              (`/Game/Blueprints/FrostbittenGameInst_BP.SavePlayerData` (`self.GameInstance`))
              (`GameplayStatics.OpenLevel` "Backyard"))))
        (:`B`
          (goto _label :!via `Reverse`)))
      (else
        (`GameplayStatics.PlaySound2D` "/Game/Audio/SFX/SFX_LockedDoor.SFX_LockedDoor" 1.0 1.0 0.0 null null)))))

(event `self.Box.OnComponentBeginOverlap`
  (params (OverlappedComponent :type "PrimitiveComponent Object Reference") (OtherActor :type "Actor Object Reference") (OtherComp :type "PrimitiveComponent Object Reference") (OtherBodyIndex :type Integer) (bFromSweep :type Boolean) (SweepResult :type "HitResult Structure (by ref)"))
  (cast `/Game/Player_Content/Player` OtherActor)
  (`self.EnableInput` (`GameplayStatics.GetPlayerController` 0)))

(event `self.Box.OnComponentEndOverlap`
  (params (OverlappedComponent :type "PrimitiveComponent Object Reference") (OtherActor :type "Actor Object Reference") (OtherComp :type "PrimitiveComponent Object Reference") (OtherBodyIndex :type Integer))
  (cast `/Game/Player_Content/Player` OtherActor)
  (`self.DisableInput` (`GameplayStatics.GetPlayerController` 0)))

(fn `UserConstructionScript`)