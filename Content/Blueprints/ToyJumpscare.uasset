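; ToyJumpscare is a trap actor, a lit toy that triggers a Frost jumpscare and sends the player to HouseMap.
; The first overlap on its collider plays a roar and animation, then reveals the skeletal mesh as the toy and point light are destroyed.
; After a short hold it saves player data through FrostbittenGameInst_BP and opens the level.
; Play-rate and component-move nodes are left unconnected.
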(event `self.Collider.OnComponentBeginOverlap`
  (params (OverlappedComponent :type "PrimitiveComponent Object Reference") (OtherActor :type "Actor Object Reference") (OtherComp :type "PrimitiveComponent Object Reference") (OtherBodyIndex :type Integer) (bFromSweep :type Boolean) (SweepResult :type "HitResult Structure (by ref)"))
  (`/Engine/EditorBlueprintResources/StandardMacros.DoOnce` false
    (:`Completed`
      (`self.Jumpscare`))))

(event `Jumpscare`
  (bind _fs_jumpscareskeletal (`self.FS_JumpscareSkeletal`))
  (`GameplayStatics.PlaySound2D` "/Game/Audio/SFX_FrostRoar_main.SFX_FrostRoar_main" 1.0 1.0 0.0 null null)
  (`SkeletalMeshComponent.PlayAnimation` _fs_jumpscareskeletal "/Game/Levels/Assets/Gary/FrostStalkerGaryAnims/Frost_Bed_Short.Frost_Bed_Short" false)
  (`KismetSystemLibrary.Delay` 0.2)
  (`SceneComponent.SetVisibility` _fs_jumpscareskeletal true false)
  (`ActorComponent.K2_DestroyComponent` (`self.Toy`))
  (`ActorComponent.K2_DestroyComponent` (`self.PointLight`))
  (`KismetSystemLibrary.Delay` 1.0)
  (bind _asfrostbitten_game_inst_bp (cast `/Game/Blueprints/FrostbittenGameInst_BP` (`GameplayStatics.GetGameInstance`)))
  (`/Game/Blueprints/FrostbittenGameInst_BP.SavePlayerData` _asfrostbitten_game_inst_bp)
  (`GameplayStatics.OpenLevel` "HouseMap")
  (`self.K2_DestroyActor`))

(fn `UserConstructionScript`)