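; Gate actor that the player can unlock and swing open or closed once the game instance's HasKey flag is set.
; Collider overlap enables Interact input and shows either an unlock or need-key widget, removed on exit.
; With the key, Interact destroys the lock and FlipFlops the GateOpen timeline, which yaws the Arrow component.
; Without it, Interact plays a locked-gate voice line only once.
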(event `InputAction|Interact`
  (params (Key :type "Key Structure"))
  (:`Pressed`
    (if (`/Game/Blueprints/FrostbittenGameInst_BP.hasKey?` (stale `self.Collider.OnComponentBeginOverlap` _asfrostbitten_game_inst_bp))
      (`ActorComponent.K2_DestroyComponent` (`self.Lock`))
      (`Widget.RemoveFromParent` (stale `self.Collider.OnComponentBeginOverlap` _returnvalue))
      (`/Engine/EditorBlueprintResources/StandardMacros.FlipFlop`
        (:`A`
          (bind (_direction _door_opens) (`Timeline|Gate Open` :!label _label)
            (:`Update`
              (`SceneComponent.K2_SetRelativeRotation` (`self.Arrow`) (`KismetMathLibrary.MakeRotator` 0.0 0.0 (* _door_opens (`self.Angle`))) false false))))
        (:`B`
          (goto _label :!via `Reverse`)))
      (else
        (`/Engine/EditorBlueprintResources/StandardMacros.DoOnce` false
          (:`Completed`
            (`GameplayStatics.PlaySound2D` "/Game/Audio/Voice/Dial_Thomas_damn_thing_is_locked.Dial_Thomas_damn_thing_is_locked" 1.0 1.0 0.0 null null)))))))

(event `self.Collider.OnComponentBeginOverlap`
  (params (OverlappedComponent :type "PrimitiveComponent Object Reference") (OtherActor :type "Actor Object Reference") (OtherComp :type "PrimitiveComponent Object Reference") (OtherBodyIndex :type Integer) (bFromSweep :type Boolean) (SweepResult :type "HitResult Structure (by ref)"))
  (if (== OtherActor (`GameplayStatics.GetPlayerPawn` 0))
    (bind _asfrostbitten_game_inst_bp (cast `/Game/Blueprints/FrostbittenGameInst_BP` (`GameplayStatics.GetGameInstance`)))
    (`self.EnableInput` (`GameplayStatics.GetPlayerController` 0))
    (if (`/Game/Blueprints/FrostbittenGameInst_BP.hasKey?` _asfrostbitten_game_inst_bp)
      (`/Engine/EditorBlueprintResources/StandardMacros.DoOnce` false :!label _label_2
        (:`Completed`
          (bind _returnvalue (`|CreateWidget` "/Game/Blueprints/Widgets/PressEtoUnlock_BP.PressEtoUnlock_BP_C"))
          (`UserWidget.AddToViewport` _returnvalue 0)))
      (else
        (`/Engine/EditorBlueprintResources/StandardMacros.DoOnce` false :!label _label_3
          (:`Completed`
            (bind _returnvalue_2 (`|CreateWidget` "/Game/Blueprints/Widgets/YouNeedKey_BP.YouNeedKey_BP_C"))
            (`UserWidget.AddToViewport` _returnvalue_2 0)))))))

(event `self.Collider.OnComponentEndOverlap`
  (params (OverlappedComponent :type "PrimitiveComponent Object Reference") (OtherActor :type "Actor Object Reference") (OtherComp :type "PrimitiveComponent Object Reference") (OtherBodyIndex :type Integer))
  (if (== OtherActor (`GameplayStatics.GetPlayerPawn` 0))
    (bind _asfrostbitten_game_inst_bp (cast `/Game/Blueprints/FrostbittenGameInst_BP` (`GameplayStatics.GetGameInstance`)))
    (`self.DisableInput` (`GameplayStatics.GetPlayerController` 0))
    (if (`/Game/Blueprints/FrostbittenGameInst_BP.hasKey?` _asfrostbitten_game_inst_bp)
      (`Widget.RemoveFromParent` (stale `self.Collider.OnComponentBeginOverlap` _returnvalue))
      (goto _label_2 :!via `Reset`)
      (else
        (`Widget.RemoveFromParent` (stale `self.Collider.OnComponentBeginOverlap` _returnvalue_2))
        (goto _label_3 :!via `Reset`)))))

(fn `UserConstructionScript`)