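; Trigger volume that stages the Josh apparition "blink and miss it" event as the player passes through.
; The first player overlap sets the Player's Danger flag.
; Each player exit removes the Blink widget, and a DoOnce fires the player's blink component, calls BlinkAndMissIt on the JoshApparition_BP found by class lookup, and clears Danger.
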(event `self.Trigger.OnComponentBeginOverlap`
  (params (OverlappedComponent :type "PrimitiveComponent Object Reference") (OtherActor :type "Actor Object Reference") (OtherComp :type "PrimitiveComponent Object Reference") (OtherBodyIndex :type Integer) (bFromSweep :type Boolean) (SweepResult :type "HitResult Structure (by ref)"))
  (if (== (`GameplayStatics.GetPlayerPawn` 0) OtherActor)
    (`/Engine/EditorBlueprintResources/StandardMacros.DoOnce` false
      (:`Completed`
        (bind _returnvalue (`GameplayStatics.GetActorOfClass` "/Game/Player_Content/Player.Player_C"))
        (set `/Game/Player_Content/Player.Danger?` true _returnvalue)))))

(event `self.Trigger.OnComponentEndOverlap`
  (params (OverlappedComponent :type "PrimitiveComponent Object Reference") (OtherActor :type "Actor Object Reference") (OtherComp :type "PrimitiveComponent Object Reference") (OtherBodyIndex :type Integer))
  (if (== OtherActor (`GameplayStatics.GetPlayerPawn` 0))
    (`Widget.RemoveFromParent` (`self.Blink`))
    (`/Engine/EditorBlueprintResources/StandardMacros.DoOnce` (`self.Start Closed`)
      (:`Completed`
        (bind _returnvalue (`GameplayStatics.GetActorOfClass` "/Game/Player_Content/Player.Player_C"))
        (`/Game/Blueprints/BlinkComponent_BP.Blinks` (`/Game/Player_Content/Player.BlinkComponent_BP` _returnvalue))
        (bind _returnvalue_2 (`GameplayStatics.GetActorOfClass` "/Game/Blueprints/JoshApparition/JoshApparition_BP.JoshApparition_BP_C"))
        (`/Game/Blueprints/JoshApparition/JoshApparition_BP.BlinkAndMissIt` _returnvalue_2)
        (set `/Game/Player_Content/Player.Danger?` false _returnvalue)))))

(fn `UserConstructionScript`)