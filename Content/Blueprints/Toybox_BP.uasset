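; Toy box in Frostbitten that collects four toys and records when all of them have been turned in.
; Overlapping its collider casts for each of four MovingToy classes, setting that toy's collected flag once and destroying it.
; Tick polls the four flags and, when all are true, sets AllToysCollected on the game instance.
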(event `self.ReceiveTick`
  (params (DeltaSeconds :type "Float (single-precision)"))
  ;[1 1 1] Checks to see if player has turned in all toys then sets GameInst bool to true
  (if (and (`self.Toy1Collected?`) (`self.Toy2Collected?`) (`self.Toy3Collected?`) (`self.Toy4Collected?`))
    (bind _asfrostbitten_game_inst_bp (cast `/Game/Blueprints/FrostbittenGameInst_BP` (`GameplayStatics.GetGameInstance`)))
    (bind _output_get (set `/Game/Blueprints/FrostbittenGameInst_BP.AllToysCollected?` true _asfrostbitten_game_inst_bp))
    (if _output_get
      (`/Engine/EditorBlueprintResources/StandardMacros.DoOnce` false))))

(event `self.Collider.OnComponentBeginOverlap`
  (params (OverlappedComponent :type "PrimitiveComponent Object Reference") (OtherActor :type "Actor Object Reference") (OtherComp :type "PrimitiveComponent Object Reference") (OtherBodyIndex :type Integer) (bFromSweep :type Boolean) (SweepResult :type "HitResult Structure (by ref)"))
  ;[1 1 1] Checks to see if each toy has been put inside, when one does, a specific bool gets set to true and toy gets destroyed
  (`|ExecutionSequence`
    (:`then_0`
      (bind _asmoving_toy (cast `/Game/Blueprints/MovingToy` OtherActor))
      (`/Engine/EditorBlueprintResources/StandardMacros.DoOnce` false
        (:`Completed`
          (set `self.Toy1Collected?` true)
          (`self.K2_DestroyActor` _asmoving_toy))))
    (:`then_1`
      (bind _asmoving_toy_2 (cast `/Game/Blueprints/MovingToy2` OtherActor))
      (`/Engine/EditorBlueprintResources/StandardMacros.DoOnce` false
        (:`Completed`
          (set `self.Toy2Collected?` true)
          (`self.K2_DestroyActor` _asmoving_toy_2))))
    (:`then_2`
      (bind _asmoving_toy_3 (cast `/Game/Blueprints/MovingToy3` OtherActor))
      (`/Engine/EditorBlueprintResources/StandardMacros.DoOnce` false
        (:`Completed`
          (set `self.Toy3Collected?` true)
          (`self.K2_DestroyActor` _asmoving_toy_3))))
    (:`then_3`
      (bind _asmoving_toy_4 (cast `/Game/Blueprints/MovingToy4` OtherActor))
      (`/Engine/EditorBlueprintResources/StandardMacros.DoOnce` false
        (:`Completed`
          (set `self.Toy4Collected?` true)
          (`self.K2_DestroyActor` _asmoving_toy_4))))))

(fn `UserConstructionScript`)