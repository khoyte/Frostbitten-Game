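; Key pickup encased in ice, which the player burns away by holding Interact while inside the collider.
; Overlap enables input, shows a hold-E progress widget and opens a gate; leaving reverses this.
; A press starts a retriggerable delay plus a timer that a recursive update polls to fill the widget.
; If still held afterwards, it grants the key to player and game instance, adds an objective, saves the respawn transform and destroys itself.
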(event `InputAction|Interact`
  (params (Key :type "Key Structure"))
  ;[1 1 1] Checks to see if player is holding E and displays widget
  (:`Pressed`
    (set `self.IsHeld?` true)
    (`GameplayStatics.PlaySound2D` "/Game/Audio/SFX_Lighter.SFX_Lighter" 1.0 1.0 0.0 null null)
    (`/Engine/EditorBlueprintResources/StandardMacros.Gate` true :!label _label
      (:`Exit`
        ;[1 1 1] If Player held E and burnt the ice then player recieves key
        (`|ExecutionSequence`
          (:`then_0`
            (`KismetSystemLibrary.RetriggerableDelay` (`self.MaxHoldTime`))
            (if (`self.IsHeld?`)
              (bind _asfrostbitten_game_inst_bp (cast `/Game/Blueprints/FrostbittenGameInst_BP` (`GameplayStatics.GetGameInstance`)))
              (bind _asplayer (cast `/Game/Player_Content/Player` (`GameplayStatics.GetPlayerCharacter` 0)))
              (set `/Game/Player_Content/Player.HasKey?` true _asplayer)
              (set `/Game/Blueprints/FrostbittenGameInst_BP.hasKey?` true _asfrostbitten_game_inst_bp)
              (`GameplayStatics.PlaySound2D` "/Game/Audio/Voice/Campgrounds/Dial_CG5.Dial_CG5" 1.0 1.0 0.0 null null)
              (bind _asplayer_2 (cast `/Game/Player_Content/Player` (stale `self.Collider.OnComponentBeginOverlap` OtherActor)))
              (bind _asfrostbitten_gm (cast `/Game/Blueprints/FrostbittenGM` (`GameplayStatics.GetGameMode`)))
              (`/Game/Player_Content/Player.AddObjective` _asplayer_2 (`self.Objective`))
              (set `/Game/Blueprints/FrostbittenGM.Spawn Transform` (`self.GetTransform` _asplayer_2) _asfrostbitten_gm)
              (`ActorComponent.K2_DestroyComponent` (`self.Ice`))
              (`self.K2_DestroyActor`)))
          (:`then_1`
            (`self.Timer`)
            (`self.UpdateTimer`))))))
  (:`Released`
    (set `self.IsHeld?` false)))

(event `self.Collider.OnComponentBeginOverlap`
  (params (OverlappedComponent :type "PrimitiveComponent Object Reference") (OtherActor :type "Actor Object Reference") (OtherComp :type "PrimitiveComponent Object Reference") (OtherBodyIndex :type Integer) (bFromSweep :type Boolean) (SweepResult :type "HitResult Structure (by ref)"))
  ;[1 1 1] Checks to see if player is holding E and displays widget
  (cast `/Game/Player_Content/Player` OtherActor)
  (`self.EnableInput` (`GameplayStatics.GetPlayerController` 0))
  (`/Engine/EditorBlueprintResources/StandardMacros.DoOnce` false :!label _label_2
    (:`Completed`
      (bind _returnvalue (`|CreateWidget` "/Game/Blueprints/Widgets/HoldEKeyWidget_BP.HoldEKeyWidget_BP_C"))
      (bind _output_get (set `self.KeyWidgetREF` _returnvalue))
      (`UserWidget.AddToViewport` _output_get 0)
      (set `/Game/Blueprints/Widgets/HoldEKeyWidget_BP.MaxTimeHeld` (`self.MaxHoldTime`) _returnvalue)
      (goto _label :!via `Open`))))

(event `self.Collider.OnComponentEndOverlap`
  (params (OverlappedComponent :type "PrimitiveComponent Object Reference") (OtherActor :type "Actor Object Reference") (OtherComp :type "PrimitiveComponent Object Reference") (OtherBodyIndex :type Integer))
  ;[1 1 1] Checks to see if player is holding E and displays widget
  (cast `/Game/Player_Content/Player` OtherActor)
  (`self.DisableInput` (`GameplayStatics.GetPlayerController` 0))
  (`Widget.RemoveFromParent` (stale `self.Collider.OnComponentBeginOverlap` _returnvalue))
  (`|ExecutionSequence`
    (:`then_0`
      (goto _label_2 :!via `Reset`))
    (:`then_1`
      (goto _label :!via `Close`))
    (:`then_2`
      (`self.StopTimer`)
      (set `/Game/Blueprints/Widgets/HoldEKeyWidget_BP.TimeHeld` 0.0 (`self.KeyWidgetREF`))
      (set `self.IsHeld?` false))))

(event `StopTimer`
  ;[1 1 1] Timer Logic for burning
  (`KismetSystemLibrary.K2_PauseTimerHandle` (stale `Timer` _returnvalue)))

(event `Timer`
  ;[1 1 1] Timer Logic for burning
  (bind _returnvalue (`KismetSystemLibrary.K2_SetTimerDelegate` (delegate `Timer`) (`self.MaxHoldTime`))))

(event `UpdateTimer`
  (bind _keywidgetref (`self.KeyWidgetREF`))
  ;[1 1 1] Timer Logic for burning
  (if (`self.IsHeld?`)
    (set `/Game/Blueprints/Widgets/HoldEKeyWidget_BP.TimeHeld` (`KismetSystemLibrary.K2_GetTimerElapsedTimeHandle` (stale `Timer` _returnvalue)) _keywidgetref)
    (`KismetSystemLibrary.Delay` 0.1)
    (`self.UpdateTimer`)
    (else
      (`self.StopTimer`)
      (set `/Game/Blueprints/Widgets/HoldEKeyWidget_BP.TimeHeld` 0.0 _keywidgetref))))

(fn `UserConstructionScript`)