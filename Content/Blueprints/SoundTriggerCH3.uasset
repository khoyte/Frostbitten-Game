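; SoundTriggerCH3 is a trigger actor that plays a 2D sound when the player enters its box while carrying the jerry can.
; The HasJerryCan flag is read from the Frostbitten game instance, cached on BeginPlay.
; A DoOnce limits the sound to a single play.
; A DontPlay event can suppress the trigger for twenty seconds before clearing itself.
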(event `self.ReceiveBeginPlay`
  (bind _asfrostbitten_game_inst_bp (cast `/Game/Blueprints/FrostbittenGameInst_BP` (`GameplayStatics.GetGameInstance`)))
  (set `self.GameInst` _asfrostbitten_game_inst_bp))

(event `self.Box.OnComponentBeginOverlap`
  (params (OverlappedComponent :type "PrimitiveComponent Object Reference") (OtherActor :type "Actor Object Reference") (OtherComp :type "PrimitiveComponent Object Reference") (OtherBodyIndex :type Integer) (bFromSweep :type Boolean) (SweepResult :type "HitResult Structure (by ref)"))
  (cast `/Game/Player_Content/Player` OtherActor)
  (if (`/Game/Blueprints/FrostbittenGameInst_BP.HasJerryCan?` (`self.GameInst`))
    (if (not (`self.Don't Play`))
      (`/Engine/EditorBlueprintResources/StandardMacros.DoOnce` false
        (:`Completed`
          (`GameplayStatics.PlaySound2D` (`self.Sound`) 1.0 1.0 0.0 null null))))))

(event `DontPlay`
  (set `self.Don't Play` true)
  (`KismetSystemLibrary.Delay` 20.0)
  (set `self.Don't Play` false))

(fn `UserConstructionScript`)