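; Locker door Blueprint that lets the player hide inside a locker and climb back out with the Interact input.
; A box overlap enables input, shows a tutorial widget and plays a delayed dialogue sound.
; Entering plays a sequence, starts a heartbeat, switches view to the Locker_Edit_Blueprint actor and teleports the hidden player to a hard-coded location.
; Exiting plays another sequence, restores view, visibility and saved position, then adds an objective.
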(event `InputAction|Interact`
  (params (Key :type "Key Structure"))
  (bind _returnvalue (`GameplayStatics.GetPlayerController` 0))
  (bind _returnvalue_2 (`GameplayStatics.GetPlayerCharacter` 0))
  (bind _returnvalue_3 (`GameplayStatics.GetPlayerController` 0))
  (bind _returnvalue_4 (`GameplayStatics.GetPlayerController` 0))
  (bind _capsulecomponent (`Character.CapsuleComponent` _returnvalue_2))
  (bind _mesh (`Character.Mesh` _returnvalue_2))
  ;[1 1 1] Open/Close door
  (:`Pressed`
    (if (`self.InsideLocker`)
      (`self.DisableInput` _returnvalue)
      (`self.DisableInput` (`GameplayStatics.GetPlayerCharacter` 0) _returnvalue)
      (set `self.InsideLocker` false)
      (`ActorComponent.SetActive` (stale _returnvalue_6) false false)
      (`MovieSceneSequencePlayer.Play` (`self.ExitLocker`))
      (`KismetSystemLibrary.Delay` 4.5)
      (`self.EnableInput` _returnvalue_2 _returnvalue_3)
      (`PlayerController.SetViewTargetWithBlend` _returnvalue_3 _returnvalue_2 0.0 "VTBlend_Linear" 0.0 false)
      (`SceneComponent.SetVisibility` _mesh true false)
      (`SceneComponent.K2_SetWorldLocation` _capsulecomponent (`self.Return`) false true)
      (bind _returnvalue_5 (`GameplayStatics.GetActorOfClass` "/Game/Player_Content/Player.Player_C"))
      (`/Game/Player_Content/Player.AddObjective` _returnvalue_5 (`self.Objective`))
      (elif (`self.Overlapped`)
        (`self.DisableInput` _returnvalue_4)
        (`self.DisableInput` (`GameplayStatics.GetPlayerCharacter` 0) _returnvalue_4)
        (`MovieSceneSequencePlayer.Play` (`self.EnterLocker`))
        (`SceneComponent.SetVisibility` _mesh false false)
        (`KismetSystemLibrary.Delay` 4.9)
        (set `self.InsideLocker` true)
        (bind _returnvalue_6 (`GameplayStatics.SpawnSound2D` (`self.HeartBeatSFX`) 1.0 1.0 0.0 null))
        (`ActorComponent.SetActive` _returnvalue_6 true false)
        (`self.EnableInput` _returnvalue_3)
        (bind _returnvalue_7 (`GameplayStatics.GetActorOfClass` "/Game/Blueprints/Locker_Edit_Blueprint.Locker_Edit_Blueprint_C"))
        (`PlayerController.SetViewTargetWithBlend` _returnvalue_3 _returnvalue_7 0.0 "VTBlend_Linear" 0.0 false)
        (bind _outactors (`GameplayStatics.GetAllActorsOfClass` "/Game/Blueprints/SpawnTarget.SpawnTarget_C"))
        (set `self.Return` (`SceneComponent.K2_GetComponentLocation` _capsulecomponent))
        (`SceneComponent.K2_SetWorldLocation` _capsulecomponent (5324.504883 33599.101562 3429.198486) false true)
        (`self.K2_AddActorWorldRotation` _returnvalue_2 (struct :`Yaw` -180.0) false false)))))

(event `self.Box.OnComponentBeginOverlap`
  (params (OverlappedComponent :type "PrimitiveComponent Object Reference") (OtherActor :type "Actor Object Reference") (OtherComp :type "PrimitiveComponent Object Reference") (OtherBodyIndex :type Integer) (bFromSweep :type Boolean) (SweepResult :type "HitResult Structure (by ref)"))
  ;[1 1 1] Interact Door Overlap
  (cast `/Game/Player_Content/Player` OtherActor)
  (`self.EnableInput` (`GameplayStatics.GetPlayerController` 0))
  (`/Engine/EditorBlueprintResources/StandardMacros.DoOnce` false :!label _label
    (:`Completed`
      (bind _returnvalue (`|CreateWidget` "/Game/Blueprints/Widgets/Tutorials/InteractTutorial_BP.InteractTutorial_BP_C"))
      (bind _output_get (set `self.Interact` _returnvalue))
      (`UserWidget.AddToViewport` _output_get 0)
      (set `self.Overlapped` true)
      (`/Engine/EditorBlueprintResources/StandardMacros.DoOnce` false
        (:`Completed`
          (`KismetSystemLibrary.Delay` 15.0)
          (`GameplayStatics.PlaySound2D` "/Game/Audio/Voice/Watchtower/Dial_WT5.Dial_WT5" 1.0 1.0 0.0 null null))))))

(event `self.Box.OnComponentEndOverlap`
  (params (OverlappedComponent :type "PrimitiveComponent Object Reference") (OtherActor :type "Actor Object Reference") (OtherComp :type "PrimitiveComponent Object Reference") (OtherBodyIndex :type Integer))
  ;[1 1 1] Interact Door Overlap
  (if (not (`self.InsideLocker`))
    (cast `/Game/Player_Content/Player` OtherActor)
    (`self.DisableInput` (`GameplayStatics.GetPlayerController` 0))
    (`Widget.RemoveFromParent` (`self.Interact`))
    (set `self.Overlapped` false)
    (goto _label :!via `Reset`)))

(event `self.ReceiveBeginPlay`
  (bind (_outactor _returnvalue) (`LevelSequencePlayer.CreateLevelSequencePlayer` "/Game/UI/Cinematics/LockerEnterCutscene.LockerEnterCutscene"))
  (set `self.EnterLocker` _returnvalue)
  (bind (_outactor_2 _returnvalue_2) (`LevelSequencePlayer.CreateLevelSequencePlayer` "/Game/UI/Cinematics/LockerExitCutscene.LockerExitCutscene"))
  (set `self.ExitLocker` _returnvalue_2))

(event `self.ExitLocker.OnFinished`
  (`self.EnableInput` (`GameplayStatics.GetPlayerCharacter` 0) (`GameplayStatics.GetPlayerController` 0) :!label _label_2))

(event `self.EnterLocker.OnFinished`
  (goto _label_2))

(fn `UserConstructionScript`)