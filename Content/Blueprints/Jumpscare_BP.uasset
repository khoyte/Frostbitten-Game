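; Trigger-volume jumpscare actor that springs a Frost Stalker on the player, armed only after the player has heard the voicemail.
; On overlap it fires once, revealing the creature with a sound and a sped-up walk animation while MoveComponentTo lunges it along its relative X.
; A second sound follows shortly after, and the actor hides the creature and destroys itself once the jumpscare duration ends.
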(event `self.Collider.OnComponentBeginOverlap`
  (params (OverlappedComponent :type "PrimitiveComponent Object Reference") (OtherActor :type "Actor Object Reference") (OtherComp :type "PrimitiveComponent Object Reference") (OtherBodyIndex :type Integer) (bFromSweep :type Boolean) (SweepResult :type "HitResult Structure (by ref)"))
  (bind _froststalker (`self.FrostStalker`))
  (bind _relativelocation (`SceneComponent.RelativeLocation` _froststalker))
  (bind _asplayer (cast `/Game/Player_Content/Player` OtherActor))
  (if (`/Game/Player_Content/Player.HeardVoicemail?` _asplayer)
    (`/Engine/EditorBlueprintResources/StandardMacros.DoOnce` false
      (:`Completed`
        (`SceneComponent.SetVisibility` (`self.FrostStalker`) true false)
        (`GameplayStatics.PlaySound2D` (`self.Jumpscare Sound`) 1.0 1.0 0.0 null null)
        (`SkeletalMeshComponent.PlayAnimation` _froststalker "/Game/Levels/Assets/Anna/New_Frost_Stalker_Anims/Frost_Stalker_Animations_17_Anim_Walk_1.Frost_Stalker_Animations_17_Anim_Walk_1" false)
        (`SkeletalMeshComponent.SetPlayRate` _froststalker 3.0)
        (`KismetSystemLibrary.MoveComponentTo` _froststalker (`KismetMathLibrary.VInterpTo` _relativelocation (+ _relativelocation (500.0 0.0 0.0))) (struct :`Yaw` -90.0) false true 0.8)
        (`|ExecutionSequence`
          (:`then_0`
            (`KismetSystemLibrary.Delay` (`self.Jumpscare Duration`))
            (`SceneComponent.SetVisibility` (`self.FrostStalker`) false false)
            (`self.K2_DestroyActor`))
          (:`then_1`
            (`KismetSystemLibrary.Delay` 0.5)
            (`GameplayStatics.PlaySound2D` "/Game/Audio/Voice/Campgrounds/Dial_CG9.Dial_CG9" 1.0 1.0 0.0 null null)))))))

(fn `UserConstructionScript`)