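; Checkpoint trigger that saves progress when the Player enters its collider.
; A DoOnce limits it to the first player overlap, which calls SavePlayerData on the Frostbitten game instance, then CallCheckPointReached on the game state.
; An unconnected branch that would store the player's transform as the GameMode spawn point never runs.
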(event `self.Collider.OnComponentBeginOverlap`
  (params (OverlappedComponent :type "PrimitiveComponent Object Reference") (OtherActor :type "Actor Object Reference") (OtherComp :type "PrimitiveComponent Object Reference") (OtherBodyIndex :type Integer) (bFromSweep :type Boolean) (SweepResult :type "HitResult Structure (by ref)"))
  (bind _asplayer (cast `/Game/Player_Content/Player` OtherActor))
  (`/Engine/EditorBlueprintResources/StandardMacros.DoOnce` false
    (:`Completed`
      (bind _asfrostbitten_game_inst_bp (cast `/Game/Blueprints/FrostbittenGameInst_BP` (`GameplayStatics.GetGameInstance`)))
      (`/Game/Blueprints/FrostbittenGameInst_BP.SavePlayerData` _asfrostbitten_game_inst_bp)
      (bind _asfrostbitten_game_state (cast `/Game/Blueprints/SaveGame/FrostbittenGameState` (`GameplayStatics.GetGameState`)))
      (`/Game/Blueprints/SaveGame/FrostbittenGameState.CheckPointReached` _asfrostbitten_game_state))))

(fn `UserConstructionScript`)