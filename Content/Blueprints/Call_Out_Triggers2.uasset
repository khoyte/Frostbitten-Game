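; A call-out trigger volume that advances the player's location progress and answers call-outs with a giggle sound.
; Player overlap at a Locations count of 2 increments it once, adds an objective, then calls SpawnFS only if the count reads 4.
; A separate Response event plays the attenuated giggles at the trigger's collision component, then finds the Player actor and ends its call-out.
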(event `Response'`
  ;[1 1 1] Call Out Respond
  (`GameplayStatics.PlaySoundAtLocation` "/Game/Blueprints/Giggles.Giggles" (`SceneComponent.K2_GetComponentLocation` (`self.CollisionComponent`)) (struct) 1.3 1.0 0.0 "/Game/Blueprints/PlayerAttenuation.PlayerAttenuation" null null)
  (bind _returnvalue (`GameplayStatics.GetActorOfClass` "/Game/Player_Content/Player.Player_C"))
  (`/Game/Player_Content/Player.End Call Out` _returnvalue))

(event `self.CollisionComponent.OnComponentBeginOverlap`
  (params (OverlappedComponent :type "PrimitiveComponent Object Reference") (OtherActor :type "Actor Object Reference") (OtherComp :type "PrimitiveComponent Object Reference") (OtherBodyIndex :type Integer) (bFromSweep :type Boolean) (SweepResult :type "HitResult Structure (by ref)"))
  (bind _asplayer (cast `/Game/Player_Content/Player` OtherActor))
  (bind _locations (`/Game/Player_Content/Player.locations` _asplayer))
  (if (== _locations 2)
    (`/Engine/EditorBlueprintResources/StandardMacros.DoOnce` false
      (:`Completed`
        (bind _output_get (set `/Game/Player_Content/Player.locations` (+ _locations 1) _asplayer))
        (`/Game/Player_Content/Player.AddObjective` _asplayer (`self.Objective`))
        (if (== _output_get 4)
          (`/Game/Player_Content/Player.Spawn FS'` _asplayer))))))

(fn `UserConstructionScript`)