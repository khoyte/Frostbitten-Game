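; Frostbitten's game instance, holding player progress, inventory and story flags and handling their save slots.
; LoadGame loads or creates a FrostSaveGameObject for the chosen slot, and LoadPlayerData copies its PlayerData into instance variables.
; SavePlayerData writes those variables back to the slot, recording ThomasStation as the level when saving from the main menu.
; Helpers edit the inventory array, read any slot's data without applying it, and delete slots.
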(event `AddArrayElement`
  (params (ItemInfo :type "/Game/Player_Content/Item_Info_Structure Structure"))
  (`KismetArrayLibrary.Array_Add` (`self.InventoryData`) ItemInfo))

(event `RemoveArrayElement`
  (params (ItemInfo :type "/Game/Player_Content/Item_Info_Structure Structure"))
  (`KismetArrayLibrary.Array_RemoveItem` (`self.InventoryData`) ItemInfo))

(event `LoadGame`
  (params (SaveSlotName :type String))
  (bind _output_get (set `self.SaveSlotName` SaveSlotName))
  (bind _returnvalue (`GameplayStatics.DoesSaveGameExist` _output_get))
  (if _returnvalue
    (bind _returnvalue_2 (`GameplayStatics.LoadGameFromSlot` (`self.SaveSlotName`)))
    (bind _asfrost_save_game_object (cast `/Game/Blueprints/SaveGame/FrostSaveGameObject` _returnvalue_2))
    (set `self.SaveGameData` _asfrost_save_game_object)
    (else
      (bind _returnvalue_3 (`GameplayStatics.CreateSaveGameObject` "/Game/Blueprints/SaveGame/FrostSaveGameObject.FrostSaveGameObject_C"))
      (set `self.SaveGameData` _returnvalue_3))))

(fn `ClearSaveData`
  (`GameplayStatics.DeleteGameInSlot` (`self.SaveSlotName`)))

(fn `ClearSaveDataMainMenu`
  (params (SlotName :type String))
  (`GameplayStatics.DeleteGameInSlot` SlotName))

(fn `LoadPlayerData`
  (locals (`Player Reference` :type "/Game/Player_Content/Player Object Reference"))
  (bind _savegamedata (`self.SaveGameData`)
    (:`then`
      (bind (_playerdata_lives _playerdata_froskrscollected _playerdata_levelname _playerdata_inventory _playerdata_hasvoicemail_ _playerdata_hasgatekey_ _playerdata_holdsprint_ _playerdata_readjournal _playerdata_hasjerrycan) (break `/Game/Blueprints/SaveGame/PlayerSaveData` (`/Game/Blueprints/SaveGame/FrostSaveGameObject.PlayerData` _savegamedata)))
      (set `self.Lives` _playerdata_lives)
      (set `self.FroskrsCollected` _playerdata_froskrscollected)
      (set `self.LevelName` _playerdata_levelname)
      (set `self.InventoryData` _playerdata_inventory)
      (set `self.hasVoicemail?` _playerdata_hasvoicemail_)
      (set `self.hasKey?` _playerdata_hasgatekey_)
      (set `self.HoldSprint?` _playerdata_holdsprint_)
      (set `self.ReadJournal?` _playerdata_readjournal)
      (set `self.HasJerryCan?` _playerdata_hasjerrycan))
    (:`else`)))

(fn `Retrieve Save Data`
  (params (LocalSaveSlotName :type String))
  (returns (PlayerData :type "/Game/Blueprints/SaveGame/PlayerSaveData Structure"))
  (bind _returnvalue (`GameplayStatics.DoesSaveGameExist` LocalSaveSlotName))
  (if _returnvalue
    (bind _returnvalue_2 (`GameplayStatics.LoadGameFromSlot` (`local.LocalSaveSlotName`)))
    (bind _asfrost_save_game_object (cast `/Game/Blueprints/SaveGame/FrostSaveGameObject` _returnvalue_2))
    (return (`/Game/Blueprints/SaveGame/FrostSaveGameObject.PlayerData` _asfrost_save_game_object))))

(fn `SavePlayerData`
  (locals (`Player Refrence` :type "/Game/Player_Content/Player Object Reference"))
  (bind _asplayer (cast `/Game/Player_Content/Player` (`GameplayStatics.GetPlayerCharacter` 0)))
  (set `local.Player Refrence` _asplayer)
  (bind _returnvalue (`GameplayStatics.GetCurrentLevelName` true))
  (if (`KismetStringLibrary.EqualEqual_StrStr` _returnvalue "MainMenu_Level")
    (set `self.LevelName` "ThomasStation")
    (else
      (set `self.LevelName` _returnvalue)))
  (set `/Game/Blueprints/SaveGame/FrostSaveGameObject.PlayerData` (make `/Game/Blueprints/SaveGame/PlayerSaveData` (`self.Lives`) (`self.FroskrsCollected`) (`self.LevelName`) (`self.InventoryData`) (`self.hasVoicemail?`) (`self.hasKey?`) (`self.HoldSprint?`) (`self.ReadJournal?`) (`self.HasJerryCan?`)) (`self.SaveGameData`))
  (`GameplayStatics.SaveGameToSlot` (`self.SaveGameData`) (`self.SaveSlotName`)))