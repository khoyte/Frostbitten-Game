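; Backyard hide-and-seek spawn actor that triggers the final jump scare when the player overlaps it at location stage 4.
; On overlap it disables input, flags the last hide-and-seek in the game instance and plays a jump-scare level sequence created at BeginPlay.
; After a delay it marks hide-and-seek completed, saves player data and loads the HouseMap level.
; A separate response event plays giggles and ends the player's call-out.
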(event `Response'`
  (`GameplayStatics.PlaySoundAtLocation` "/Game/Blueprints/Giggles.Giggles" (`SceneComponent.K2_GetComponentLocation` (`self.CollisionComponent`)) (struct) 1.3 1.0 0.0 "/Game/Blueprints/PlayerAttenuation.PlayerAttenuation" null null)
  (bind _returnvalue (`GameplayStatics.GetActorOfClass` "/Game/Player_Content/Player.Player_C"))
  (`/Game/Player_Content/Player.End Call Out` _returnvalue))

(event `self.ReceiveBeginPlay`
  (bind (_outactor _returnvalue) (`LevelSequencePlayer.CreateLevelSequencePlayer` "/Game/UI/Cinematics/HideSeekJumpScare.HideSeekJumpScare"))
  (set `self.JumpScare` _returnvalue))

(event `self.ReceiveActorBeginOverlap`
  (params (OtherActor :type "Actor Object Reference"))
  (bind _returnvalue (`GameplayStatics.GetPlayerController` 0))
  (bind _asplayer (cast `/Game/Player_Content/Player` OtherActor))
  (if (== (`/Game/Player_Content/Player.locations` _asplayer) 4)
    (`self.DisableInput` _asplayer _returnvalue)
    (bind _asfrostbitten_game_inst_bp (cast `/Game/Blueprints/FrostbittenGameInst_BP` (`GameplayStatics.GetGameInstance`)))
    (set `/Game/Blueprints/FrostbittenGameInst_BP.LastHideNSeek?` true _asfrostbitten_game_inst_bp)
    (`MovieSceneSequencePlayer.Play` (`self.JumpScare`))
    (`KismetSystemLibrary.Delay` 3.0)
    (set `/Game/Blueprints/FrostbittenGameInst_BP.HideNSeekCompleted?` true _asfrostbitten_game_inst_bp)
    (`/Game/Blueprints/FrostbittenGameInst_BP.SavePlayerData` _asfrostbitten_game_inst_bp)
    (`GameplayStatics.OpenLevel` "HouseMap")
    (`self.EnableInput` _asplayer _returnvalue)))

(fn `UserConstructionScript`)