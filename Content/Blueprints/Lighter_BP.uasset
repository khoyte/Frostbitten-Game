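; Lighter pickup actor that the player collects with the Interact input while inside its PickupBox.
; Player overlap enables input, shows a "press E to pick up" widget and opens a Gate; leaving reverses this.
; A DoOnce on begin overlap, reset when the player leaves, prevents repeated prompts.
; Interact through the open Gate sets HasLighter on the player, plays a 2D sound and destroys the actor.
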(event `Key|E`
  (params (Key :type "Key Structure")))

(event `InputAction|Interact`
  (params (Key :type "Key Structure"))
  (:`Pressed`
    (`/Engine/EditorBlueprintResources/StandardMacros.Gate` true :!label _label
      (:`Exit`
        (set `/Game/Player_Content/Player.HasLighter?` true (stale `self.PickupBox.OnComponentBeginOverlap` _asplayer))
        (`GameplayStatics.PlaySound2D` "/Game/Audio/Voice/Temp/Shay/JoshsStation/This_is_a_nice_lighter.This_is_a_nice_lighter" 1.0 1.0 0.0 null null)
        (`self.K2_DestroyActor`)))))

(event `self.PickupBox.OnComponentBeginOverlap`
  (params (OverlappedComponent :type "PrimitiveComponent Object Reference") (OtherActor :type "Actor Object Reference") (OtherComp :type "PrimitiveComponent Object Reference") (OtherBodyIndex :type Integer) (bFromSweep :type Boolean) (SweepResult :type "HitResult Structure (by ref)"))
  (`/Engine/EditorBlueprintResources/StandardMacros.DoOnce` false :!label _label_2
    (:`Completed`
      (bind _asplayer (cast `/Game/Player_Content/Player` OtherActor))
      (`self.EnableInput` (`GameplayStatics.GetPlayerController` 0))
      (bind _returnvalue (`|CreateWidget` "/Game/Blueprints/Widgets/PressEtoPickUp_BP.PressEtoPickUp_BP_C"))
      (`UserWidget.AddToViewport` _returnvalue 0)
      (goto _label :!via `Open`))))

(event `self.PickupBox.OnComponentEndOverlap`
  (params (OverlappedComponent :type "PrimitiveComponent Object Reference") (OtherActor :type "Actor Object Reference") (OtherComp :type "PrimitiveComponent Object Reference") (OtherBodyIndex :type Integer))
  (cast `/Game/Player_Content/Player` OtherActor)
  (`self.DisableInput` (`GameplayStatics.GetPlayerController` 0))
  (`Widget.RemoveFromParent` (stale `self.PickupBox.OnComponentBeginOverlap` _returnvalue))
  (`|ExecutionSequence`
    (:`then_0`
      (goto _label_2 :!via `Reset`))
    (:`then_1`
      (goto _label :!via `Close`))))

(fn `UserConstructionScript`)