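; Frozen house door that the player melts by holding Interact with the lighter, then saves player data and loads level VHS_4.
; Box overlap enables input and shows either a hold-E or need-lighter widget, opening a gate for the hold.
; A retriggerable delay checks the hold while a recursive timer updater feeds widget progress.
; Success swings the door by timeline and destroys the ice; once burned, Interact toggles the door through a FlipFlop.
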(event `InputAction|Interact`
  (params (Key :type "Key Structure"))
  ;[1 1 1] Allows the door to open after it burned
  (:`Pressed`
    (if (`self.BurnedIce?`)
      (`/Engine/EditorBlueprintResources/StandardMacros.FlipFlop`
        (:`A`
          (bind (_direction _door_track) (`Timeline|Timeline_1` :!label _label)
            (:`Update`
              (`SceneComponent.K2_SetRelativeRotation` (`self.Arrow`) (`KismetMathLibrary.MakeRotator` 0.0 0.0 (* _door_track (`self.Angle`))) false false))))
        (:`B`
          (goto _label :!via `Reverse`)))
      (else
        (`GameplayStatics.PlaySound2D` "/Game/Audio/SFX_Lighter.SFX_Lighter" 1.0 1.0 0.0 null null)))))

(event `InputAction|Interact`
  (params (Key :type "Key Structure"))
  ;[1 1 1] If near door, specific UI pops up
  (:`Pressed`
    (bind _output_get (set `self.IsHeld?` true))
    (`/Engine/EditorBlueprintResources/StandardMacros.Gate` true :!label _label_2
      (:`Exit`
        ;[1 1 1] If player has Lighter and holds E, plays door ani and opens/closes
        (`|ExecutionSequence`
          (:`then_0`
            (`KismetSystemLibrary.RetriggerableDelay` (`self.MaxHoldTime`))
            (if (and _output_get (`/Game/Player_Content/Player.HasLighter?` (stale `self.Box.OnComponentBeginOverlap` _asplayer)))
              (`/Engine/EditorBlueprintResources/StandardMacros.FlipFlop`
                (:`A`
                  (bind (_direction _door_track) (`Timeline|Timeline_0` :!label _label_3)
                    (:`Update`
                      (`SceneComponent.K2_SetRelativeRotation` (`self.Arrow`) (`KismetMathLibrary.MakeRotator` 0.0 0.0 (* _door_track (`self.Angle`))) false false)
                      (`Widget.RemoveFromParent` (stale `self.Box.OnComponentBeginOverlap` _returnvalue))
                      (set `self.BurnedIce?` true)
                      (`/Engine/EditorBlueprintResources/StandardMacros.DoOnce` false
                        (:`Completed`
                          (`ActorComponent.K2_DestroyComponent` (`self.Ice`))
                          ;[1 1 1] Opens HouseMap level once player melts door knob.
                          (`KismetSystemLibrary.Delay` 0.2)
                          (bind _asfrostbitten_game_inst_bp (cast `/Game/Blueprints/FrostbittenGameInst_BP` (`GameplayStatics.GetGameInstance`)))
                          (`/Game/Blueprints/FrostbittenGameInst_BP.SavePlayerData` _asfrostbitten_game_inst_bp)
                          (`GameplayStatics.OpenLevel` "VHS_4"))))))
                (:`B`
                  (goto _label_3 :!via `Reverse`)))))
          (:`then_1`
            (`self.Timer`)
            (`self.UpdateTimer`))))))
  (:`Released`
    (set `self.IsHeld?` false)))

(event `self.Box.OnComponentBeginOverlap`
  (params (OverlappedComponent :type "PrimitiveComponent Object Reference") (OtherActor :type "Actor Object Reference") (OtherComp :type "PrimitiveComponent Object Reference") (OtherBodyIndex :type Integer) (bFromSweep :type Boolean) (SweepResult :type "HitResult Structure (by ref)"))
  ;[1 1 1] If near door, specific UI pops up
  (`/Engine/EditorBlueprintResources/StandardMacros.DoOnce` false :!label _label_4
    (:`Completed`
      (bind _asplayer (cast `/Game/Player_Content/Player` OtherActor))
      (`self.EnableInput` (`GameplayStatics.GetPlayerController` 0))
      (bind _haslighter_ (`/Game/Player_Content/Player.HasLighter?` _asplayer))
      (if _haslighter_
        (if (not (and _haslighter_ (`self.BurnedIce?`)))
          (bind _returnvalue (`|CreateWidget` "/Game/Blueprints/Widgets/HoldEWidget_BP.HoldEWidget_BP_C"))
          (bind _output_get (set `self.WidgetREF` _returnvalue))
          (`UserWidget.AddToViewport` _output_get 0)
          (set `/Game/Blueprints/Widgets/HoldEWidget_BP.MaxTimeHeld` (`self.MaxHoldTime`) _output_get)
          (goto _label_2 :!via `Open`))
        (else
          (bind _returnvalue_2 (`|CreateWidget` "/Game/Blueprints/Widgets/YouNeedLighter_BP.YouNeedLighter_BP_C"))
          (`UserWidget.AddToViewport` _returnvalue_2 0))))))

(event `StopTimer`
  ;[1 1 1] Timer Functions
  (`KismetSystemLibrary.K2_PauseTimerHandle` (stale `Timer` _returnvalue)))

(event `self.Box.OnComponentEndOverlap`
  (params (OverlappedComponent :type "PrimitiveComponent Object Reference") (OtherActor :type "Actor Object Reference") (OtherComp :type "PrimitiveComponent Object Reference") (OtherBodyIndex :type Integer))
  ;[1 1 1] If near door, specific UI pops up
  (bind _asplayer (cast `/Game/Player_Content/Player` OtherActor))
  (`self.DisableInput` (`GameplayStatics.GetPlayerController` 0))
  (if (`/Game/Player_Content/Player.HasLighter?` _asplayer)
    (`Widget.RemoveFromParent` (stale `self.Box.OnComponentBeginOverlap` _returnvalue))
    (`|ExecutionSequence`
      (:`then_0`
        (goto _label_4 :!via `Reset`))
      (:`then_1`
        (goto _label_2 :!via `Close`)))
    (else
      (`Widget.RemoveFromParent` (stale `self.Box.OnComponentBeginOverlap` _returnvalue_2))
      (goto _label_4 :!via `Reset`))))

(event `Timer`
  ;[1 1 1] Timer Functions
  (bind _returnvalue (`KismetSystemLibrary.K2_SetTimerDelegate` (delegate `Timer`) (`self.MaxHoldTime`))))

(event `UpdateTimer`
  (bind _widgetref (`self.WidgetREF`))
  ;[1 1 1] Timer Functions
  (if (`self.IsHeld?`)
    (set `/Game/Blueprints/Widgets/HoldEWidget_BP.TimeHeld` (`KismetSystemLibrary.K2_GetTimerElapsedTimeHandle` (stale `Timer` _returnvalue)) _widgetref)
    (`KismetSystemLibrary.Delay` 0.1)
    (`self.UpdateTimer`)
    (else
      (`self.StopTimer`)
      (set `/Game/Blueprints/Widgets/HoldEWidget_BP.TimeHeld` 0.0 _widgetref))))

(fn `UserConstructionScript`)