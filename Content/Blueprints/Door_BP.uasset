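; Door blueprint that the player opens and closes with the Interact input while standing in its trigger box.
; Box overlaps with the Player enable or disable input on the door.
; A FlipFlop alternately plays and reverses the Door timeline, which yaws the Arrow component by the track value times Angle.
; A DoOnce, reset when the timeline finishes, plays a creak sound at the door once per swing.
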(event `InputAction|Interact`
  (params (Key :type "Key Structure"))
  (:`Pressed`
    (`/Engine/EditorBlueprintResources/StandardMacros.FlipFlop`
      (:`A`
        (bind (_direction _door_track) (`Timeline|Door` :!label _label)
          (:`Update`
            (`SceneComponent.K2_SetRelativeRotation` (`self.Arrow`) (`KismetMathLibrary.MakeRotator` 0.0 0.0 (* _door_track (`self.Angle`))) false false)
            (`/Engine/EditorBlueprintResources/StandardMacros.DoOnce` false :!label _label_2
              (:`Completed`
                (`GameplayStatics.PlaySoundAtLocation` "/Game/Audio/SFX/SFX_DoorCreak.SFX_DoorCreak" (`SceneComponent.K2_GetComponentLocation` (`self.TempDoor`)) (struct) 1.0 1.0 0.0 null null null))))
          (:`Finished`
            (goto _label_2 :!via `Reset`))))
      (:`B`
        (goto _label :!via `Reverse`)))))

(event `self.Box.OnComponentBeginOverlap`
  (params (OverlappedComponent :type "PrimitiveComponent Object Reference") (OtherActor :type "Actor Object Reference") (OtherComp :type "PrimitiveComponent Object Reference") (OtherBodyIndex :type Integer) (bFromSweep :type Boolean) (SweepResult :type "HitResult Structure (by ref)"))
  (cast `/Game/Player_Content/Player` OtherActor)
  (`self.EnableInput` (`GameplayStatics.GetPlayerController` 0)))

(event `self.Box.OnComponentEndOverlap`
  (params (OverlappedComponent :type "PrimitiveComponent Object Reference") (OtherActor :type "Actor Object Reference") (OtherComp :type "PrimitiveComponent Object Reference") (OtherBodyIndex :type Integer))
  (cast `/Game/Player_Content/Player` OtherActor)
  (`self.DisableInput` (`GameplayStatics.GetPlayerController` 0)))

(fn `UserConstructionScript`)