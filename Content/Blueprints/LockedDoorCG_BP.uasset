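; Locked door that needs a key stored in the Frostbitten game instance and leads to level VHS_2.
; Collider overlap toggles player input and shows an unlock or need-key widget based on HasDoorKey.
; Interact with the key flip-flops a Timeline that rotates the Arrow; its Update also saves player data and opens the level.
; Without the key, Interact plays a locked sound each press and a dialogue clip once.
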(event `InputAction|Interact`
  (params (Key :type "Key Structure"))
  (:`Pressed`
    (if (`/Game/Blueprints/FrostbittenGameInst_BP.hasDoorKey?` (stale `self.Collider.OnComponentBeginOverlap` _asfrostbitten_game_inst_bp))
      (`Widget.RemoveFromParent` (stale `self.Collider.OnComponentBeginOverlap` _returnvalue))
      (`/Engine/EditorBlueprintResources/StandardMacros.FlipFlop`
        (:`A`
          (bind (_direction _door_opens) (`Timeline|Timeline_0` :!label _label)
            (:`Update`
              (`SceneComponent.K2_SetRelativeRotation` (`self.Arrow`) (`KismetMathLibrary.MakeRotator` 0.0 0.0 (* _door_opens (`self.Angle`))) false false)
              (`/Game/Blueprints/FrostbittenGameInst_BP.SavePlayerData` (stale `self.Collider.OnComponentBeginOverlap` _asfrostbitten_game_inst_bp))
              (`GameplayStatics.OpenLevel` "VHS_2"))))
        (:`B`
          (goto _label :!via `Reverse`)))
      (else
        (`|ExecutionSequence`
          (:`then_0`
            (`/Engine/EditorBlueprintResources/StandardMacros.DoOnce` false
              (:`Completed`
                (`GameplayStatics.PlaySound2D` "/Game/Audio/Voice/JoshsStation/Dial_JS14.Dial_JS14" 1.0 1.0 0.0 null null))))
          (:`then_1`
            (`GameplayStatics.PlaySound2D` "/Game/Audio/SFX/SFX_LockedDoor.SFX_LockedDoor" 1.0 1.0 0.0 null null)))))))

(event `self.Collider.OnComponentBeginOverlap`
  (params (OverlappedComponent :type "PrimitiveComponent Object Reference") (OtherActor :type "Actor Object Reference") (OtherComp :type "PrimitiveComponent Object Reference") (OtherBodyIndex :type Integer) (bFromSweep :type Boolean) (SweepResult :type "HitResult Structure (by ref)"))
  (`/Engine/EditorBlueprintResources/StandardMacros.DoOnce` false :!label _label_2
    (:`Completed`
      (if (== OtherActor (`GameplayStatics.GetPlayerPawn` 0))
        (bind _asfrostbitten_game_inst_bp (cast `/Game/Blueprints/FrostbittenGameInst_BP` (`GameplayStatics.GetGameInstance`)))
        (`self.EnableInput` (`GameplayStatics.GetPlayerController` 0))
        (if (`/Game/Blueprints/FrostbittenGameInst_BP.hasDoorKey?` _asfrostbitten_game_inst_bp)
          (bind _returnvalue (`|CreateWidget` "/Game/Blueprints/Widgets/PressEtoUnlock_BP.PressEtoUnlock_BP_C"))
          (`UserWidget.AddToViewport` _returnvalue 0)
          (else
            (bind _returnvalue_2 (`|CreateWidget` "/Game/Blueprints/Widgets/YouNeedKey_BP.YouNeedKey_BP_C"))
            (`UserWidget.AddToViewport` _returnvalue_2 0)))))))

(event `self.Collider.OnComponentEndOverlap`
  (params (OverlappedComponent :type "PrimitiveComponent Object Reference") (OtherActor :type "Actor Object Reference") (OtherComp :type "PrimitiveComponent Object Reference") (OtherBodyIndex :type Integer))
  (if (== OtherActor (`GameplayStatics.GetPlayerPawn` 0))
    (bind _asfrostbitten_game_inst_bp (cast `/Game/Blueprints/FrostbittenGameInst_BP` (`GameplayStatics.GetGameInstance`)))
    (`self.DisableInput` (`GameplayStatics.GetPlayerController` 0))
    (if (`/Game/Blueprints/FrostbittenGameInst_BP.hasDoorKey?` _asfrostbitten_game_inst_bp)
      (`Widget.RemoveFromParent` (stale `self.Collider.OnComponentBeginOverlap` _returnvalue))
      (goto _label_2 :!via `Reset`)
      (else
        (`Widget.RemoveFromParent` (stale `self.Collider.OnComponentBeginOverlap` _returnvalue_2))
        (goto _label_2 :!via `Reset`)))))

(fn `UserConstructionScript`)