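; Thomas Station exit door that carries the player from this level to JoshStation.
; A Box overlap enables the door's Interact input and shows an open-prompt tutorial widget, both withdrawn on exit.
; Interact runs a Sequence: one-shot creak and car-start sounds, a black screen, a game-instance flag marking departure, and a temporary player-input lock.
; A parallel delay then saves player data through the game instance and opens the next level.
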(event `InputAction|Interact`
  (params (Key :type "Key Structure"))
  (bind _returnvalue (`GameplayStatics.GetPlayerController` 0))
  (bind _returnvalue_2 (`GameplayStatics.GetPlayerPawn` 0))
  (:`Pressed`
    (`|ExecutionSequence`
      (:`then_0`
        (`/Engine/EditorBlueprintResources/StandardMacros.DoOnce` false
          (:`Completed`
            (`GameplayStatics.PlaySoundAtLocation` "/Game/Audio/SFX/SFX_DoorCreak.SFX_DoorCreak" (`SceneComponent.K2_GetComponentLocation` (`self.TempDoor`)) (struct) 1.0 1.0 0.0 null null null))))
      (:`then_1`
        (`/Engine/EditorBlueprintResources/StandardMacros.DoOnce` false
          (:`Completed`
            (`GameplayStatics.PlaySound2D` "/Game/Audio/SFX/SFX_CarStart.SFX_CarStart" 1.0 1.0 0.0 null null))))
      (:`then_3`
        (`/Engine/EditorBlueprintResources/StandardMacros.DoOnce` false
          (:`Completed`
            (bind _returnvalue_3 (`|CreateWidget` "/Game/Blueprints/Widgets/BlackScreen.BlackScreen_C"))
            (`UserWidget.AddToViewport` _returnvalue_3 0))))
      (:`then_4`
        (bind _asfrostbitten_game_inst_bp (cast `/Game/Blueprints/FrostbittenGameInst_BP` (`GameplayStatics.GetGameInstance`)))
        (set `/Game/Blueprints/FrostbittenGameInst_BP.LeftThomasStation?` true _asfrostbitten_game_inst_bp))
      (:`then_5`
        (`self.DisableInput` _returnvalue_2 _returnvalue)
        (`KismetSystemLibrary.Delay` 5.5)
        (`self.EnableInput` _returnvalue_2 _returnvalue))
      (:`then_6`
        (`KismetSystemLibrary.Delay` 6.0)
        (bind _asfrostbitten_game_inst_bp_2 (cast `/Game/Blueprints/FrostbittenGameInst_BP` (`GameplayStatics.GetGameInstance`)))
        (`/Game/Blueprints/FrostbittenGameInst_BP.SavePlayerData` _asfrostbitten_game_inst_bp_2)
        (`GameplayStatics.OpenLevel` "JoshStation")))))

(event `self.Box.OnComponentBeginOverlap`
  (params (OverlappedComponent :type "PrimitiveComponent Object Reference") (OtherActor :type "Actor Object Reference") (OtherComp :type "PrimitiveComponent Object Reference") (OtherBodyIndex :type Integer) (bFromSweep :type Boolean) (SweepResult :type "HitResult Structure (by ref)"))
  (cast `/Game/Player_Content/Player` OtherActor)
  (`self.EnableInput` (`GameplayStatics.GetPlayerController` 0))
  (`/Engine/EditorBlueprintResources/StandardMacros.DoOnce` false :!label _label
    (:`Completed`
      (bind _returnvalue (`|CreateWidget` "/Game/Blueprints/Widgets/Tutorials/OpenTutorial_BP1.OpenTutorial_BP1_C"))
      (`UserWidget.AddToViewport` _returnvalue 0))))

(event `self.Box.OnComponentEndOverlap`
  (params (OverlappedComponent :type "PrimitiveComponent Object Reference") (OtherActor :type "Actor Object Reference") (OtherComp :type "PrimitiveComponent Object Reference") (OtherBodyIndex :type Integer))
  (cast `/Game/Player_Content/Player` OtherActor)
  (`self.DisableInput` (`GameplayStatics.GetPlayerController` 0))
  (`Widget.RemoveFromParent` (stale `self.Box.OnComponentBeginOverlap` _returnvalue))
  (goto _label :!via `Reset`))

(fn `UserConstructionScript`)