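; Trigger-style spawner that relocates the existing Frost Stalker, rather than spawning one, when the player ends overlap.
; Behind a DoOnce and a Stop flag with a delayed reset, it checks the stalker's CanMove blackboard key, teleports it to the SpawnTarget nearest the trigger, rotates it and plays a roar.
; RespawnEnemy separately moves this spawner actor itself to the TargetPoint nearest the player, using the same closest-point loop.
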(event `self.ReceiveActorEndOverlap`
  (params (OtherActor :type "Actor Object Reference"))
  (bind _new (`self.New`))
  (bind _target (`self.Target`))
  (bind _new_2 (`self.New`))
  (bind _targetspawn (`self.TargetSpawn`))
  (bind _returnvalue (`SceneComponent.K2_GetComponentLocation` (`self.CollisionComponent`)))
  ;[1 1 1] Spawn the frost stalker
  (`/Engine/EditorBlueprintResources/StandardMacros.DoOnce` false
    (:`Completed`
      (if (not (`self.Stop`))
        (cast `/Game/Player_Content/Player` OtherActor)
        (bind _returnvalue_2 (`GameplayStatics.GetActorOfClass` "/Game/Blueprints/Enemy/Alex/Frost_Stalker_BP.Frost_Stalker_BP_C"))
        (if (`BlackboardComponent.GetValueAsBool` (`AIBlueprintHelperLibrary.GetBlackboard` (`AIBlueprintHelperLibrary.GetAIController` _returnvalue_2)) "CanMove")
          (set `self.Stop` true)
          (bind _outactors (`GameplayStatics.GetAllActorsOfClass` "/Game/Blueprints/SpawnTarget.SpawnTarget_C"))
          ;[1 1 1] Get and set Target Spawn location
          (for _array_element _outactors
            (`|ExecutionSequence`
              (:`then_0`
                (`/Engine/EditorBlueprintResources/StandardMacros.DoOnce` false :!label _label
                  (:`Completed`
                    (bind _returnvalue_3 (`SceneComponent.K2_GetComponentLocation` (`/Game/Blueprints/SpawnTarget.DefaultSceneRoot` _array_element)))
                    (set `self.TargetSpawn` _returnvalue_3))))
              (:`then_1`
                (set `self.Target` (`KismetMathLibrary.VSize` (- (`self.TargetSpawn`) _returnvalue)))
                (set `self.New` (`KismetMathLibrary.VSize` (- _returnvalue_3 _returnvalue)))
                (if (< _new 0.0)
                  (set `self.New` (* _new -1.0)))
                (if (< _target 0.0)
                  (set `self.Target` (* _target -1.0)))
                (if (> (`self.Target`) _new_2)
                  (set `self.Target` _new_2)
                  (set `self.TargetSpawn` _returnvalue_3)))))
          (`self.K2_SetActorLocation` _returnvalue_2 _targetspawn false true)
          (`GameplayStatics.PlaySoundAtLocation` "/Game/Audio/FrostStalkerSounds/FrostRoar.FrostRoar" _targetspawn (struct) 1.0 1.0 0.0 null null null)
          (`self.K2_AddActorWorldRotation` _returnvalue_2 (struct :`Yaw` 180.0) false false)
          (`KismetSystemLibrary.Delay` 15.0)
          (set `self.Stop` false)
          (goto _label :!via `Reset`))))))

(event `RespawnEnemy`
  (bind _new (`self.New`))
  (bind _target (`self.Target`))
  (bind _new_2 (`self.New`))
  (bind _returnvalue (`GameplayStatics.GetActorOfClass` "/Game/Player_Content/Player.Player_C"))
  (bind _outactors (`GameplayStatics.GetAllActorsOfClass` "/Script/Engine.TargetPoint"))
  (for _array_element _outactors
    (`|ExecutionSequence`
      (:`then_0`
        (`/Engine/EditorBlueprintResources/StandardMacros.DoOnce` false :!label _label_2
          (:`Completed`
            (bind _returnvalue_2 (`SceneComponent.K2_GetComponentLocation` (`TargetPoint.ArrowComponent` _array_element)))
            (set `self.TargetSpawn` _returnvalue_2))))
      (:`then_1`
        (bind _returnvalue_3 (`self.K2_GetActorLocation` _returnvalue))
        (set `self.Target` (`KismetMathLibrary.VSize` (- (`self.TargetSpawn`) _returnvalue_3)))
        (set `self.New` (`KismetMathLibrary.VSize` (- _returnvalue_2 _returnvalue_3)))
        (if (< _new 0.0)
          (set `self.New` (* _new -1.0)))
        (if (< _target 0.0)
          (set `self.Target` (* _target -1.0)))
        (if (> (`self.Target`) _new_2)
          (set `self.Target` _new_2)
          (set `self.TargetSpawn` _returnvalue_2)))))
  (`self.K2_SetActorLocation` (`self.TargetSpawn`) false true)
  (goto _label_2 :!via `Reset`))

(fn `UserConstructionScript`)