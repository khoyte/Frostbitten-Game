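; Trigger actor that plays a three-part sound sequence, by its name a conversation, when the player enters its box.
; The box's begin-overlap event casts the other actor to Player and passes through a DoOnce, so the sequence fires only once.
; It then plays three 2D sounds in order, spaced by two variable-driven delays rather than waiting for each sound to finish.
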(event `self.Box.OnComponentBeginOverlap`
  (params (OverlappedComponent :type "PrimitiveComponent Object Reference") (OtherActor :type "Actor Object Reference") (OtherComp :type "PrimitiveComponent Object Reference") (OtherBodyIndex :type Integer) (bFromSweep :type Boolean) (SweepResult :type "HitResult Structure (by ref)"))
  (cast `/Game/Player_Content/Player` OtherActor)
  (if true
    (`/Engine/EditorBlueprintResources/StandardMacros.DoOnce` false
      (:`Completed`
        (`GameplayStatics.PlaySound2D` (`self.Sound`) 1.0 1.0 0.0 null null)
        (`KismetSystemLibrary.Delay` (`self.Duration`))
        (`GameplayStatics.PlaySound2D` (`self.Sound_0`) 1.0 1.0 0.0 null null)
        (`KismetSystemLibrary.Delay` (`self.Duration2`))
        (`GameplayStatics.PlaySound2D` (`self.Sound_1`) 1.0 1.0 0.0 null null)))))

(fn `UserConstructionScript`)