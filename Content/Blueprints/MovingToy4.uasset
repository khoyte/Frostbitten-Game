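; A toy actor that teleports whenever the player blinks, unless the player is holding this specific toy.
; BeginPlay caches the player pawn cast to Player.
; Each tick it reads the player's blink component and held flag, and a DoOnce that resets when the condition fails limits it to one instant move of TempCube per blink to a random entry in a location array.
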(event `self.ReceiveBeginPlay`
  (bind _asplayer (cast `/Game/Player_Content/Player` (`GameplayStatics.GetPlayerPawn` 0)))
  (set `self.As Player` _asplayer))

(event `self.ReceiveTick`
  (params (DeltaSeconds :type "Float (single-precision)"))
  (bind _as_player (`self.As Player`))
  ;[1 1 1] Checks to see if the player blinks and if they are not holding the specific toy, if both are true then toy teleports
  (if (and (`/Game/Blueprints/BlinkComponent_BP.Blinking` (`/Game/Player_Content/Player.BlinkComponent_BP` _as_player)) (not (`/Game/Player_Content/Player.Toy 4BeingHeld?` _as_player)))
    (`/Engine/EditorBlueprintResources/StandardMacros.DoOnce` false :!label _label
      (:`Completed`
        (`KismetSystemLibrary.MoveComponentTo` (`self.TempCube`) (`KismetArrayLibrary.Array_Random` (`self.LocationArray`)) (struct) false false 0.0)))
    (else
      (goto _label :!via `Reset`))))

(fn `UserConstructionScript`)