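; Frost Stalker watchtower enemy that patrols, chases players it sees and kills on contact.
; A chained AIMoveTo patrol walks six locations, using saved flags as entry points, then doubles back and destroys the actor.
; PawnSensing starts the chase and spotted audio; the lose-sight return to patrol is unwired.
; Contact zeroes game-instance lives and teleports it to origin; ShovelSnow_BP hits freeze it temporarily, and call-outs get an audio response.
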(event `self.ReceiveHit`
  (params (MyComp :type "PrimitiveComponent Object Reference") (Other :type "Actor Object Reference") (OtherComp :type "PrimitiveComponent Object Reference") (bSelfMoved :type Boolean) (HitLocation :type "Vector Structure") (HitNormal :type "Vector Structure") (NormalImpulse :type "Vector Structure") (Hit :type "HitResult Structure (by ref)"))
  (bind _capsulecomponent (`self.CapsuleComponent`))
  ;[1 1 1] Destroy snow mechanic
  (bind _asshovel_snow_bp (cast `/Game/Snow/SnowShovel/ShovelSnow_BP` Other))
  (`SceneComponent.SetMobility` _capsulecomponent "Static")
  (`KismetSystemLibrary.Delay` 3.0)
  (if (`/Game/Snow/SnowShovel/ShovelSnow_BP.StopMoving` _asshovel_snow_bp) :!label _label
    (`KismetSystemLibrary.Delay` 2.0)
    (goto _label)
    (else
      (`SceneComponent.SetMobility` _capsulecomponent "Movable"))))

(event `Response'`
  ;[1 1 1] Call Out Respond
  (`GameplayStatics.PlaySoundAtLocation` "/Game/Audio/SFX/Dial_FrostResponse_Alt.Dial_FrostResponse_Alt" (`SceneComponent.K2_GetComponentLocation` (`self.Mesh`)) (struct) 1.0 1.0 0.0 "/Game/Blueprints/PlayerAttenuation.PlayerAttenuation" null null)
  (bind _outactors (`GameplayStatics.GetAllActorsOfClass` "/Game/Player_Content/Player.Player_C"))
  (`/Game/Player_Content/Player.End Call Out` _outactors))

(event `self.ReceiveTick`
  (params (DeltaSeconds :type "Float (single-precision)"))
  ;[1 1 1] Constant Bone Crack sound
  (`|ExecutionSequence`
    (:`then_0`
      (`KismetSystemLibrary.Delay` 3.0)
      (`GameplayStatics.PlaySoundAtLocation` "/Game/Audio/SFX/SFX_BoneBreaking.SFX_BoneBreaking" (`SceneComponent.K2_GetComponentLocation` (`self.Mesh`)) (struct) 1.0 1.0 0.0 "/Game/Blueprints/PlayerAttenuation.PlayerAttenuation" null null))))

(event `self.ReceiveBeginPlay`
  ;[1 1 1] Create audio ref to spotted sound
  (bind _returnvalue (`AddComponent|NODE_AddAudioComponent-0`))
  (`AudioComponent.Stop` _returnvalue)
  (set `self.Audio` _returnvalue)
  (`self.Patrol`))

(event `self.HurtCollision.OnComponentBeginOverlap`
  (params (OverlappedComponent :type "PrimitiveComponent Object Reference") (OtherActor :type "Actor Object Reference") (OtherComp :type "PrimitiveComponent Object Reference") (OtherBodyIndex :type Integer) (bFromSweep :type Boolean) (SweepResult :type "HitResult Structure (by ref)"))
  (bind _fsproximityaudio (`self.FSProximityAudio`))
  ;[1 1 1] If enemy collides with player, lose 1 life and player can't move for 2 seconds (enough time for animation to play)
  (bind _asplayer (cast `/Game/Player_Content/Player` OtherActor))
  (bind _asfrostbitten_game_inst_bp (cast `/Game/Blueprints/FrostbittenGameInst_BP` (`GameplayStatics.GetGameInstance`)))
  (`/Engine/EditorBlueprintResources/StandardMacros.DoOnce` false
    (:`Completed`
      (bind _output_get (set `/Game/Blueprints/FrostbittenGameInst_BP.Lives` 0 _asfrostbitten_game_inst_bp))
      (`/Game/Blueprints/FrostbittenGameInst_BP.PlayerDied` _asfrostbitten_game_inst_bp)
      (`KismetSystemLibrary.Delay` 0.1)
      (`|ExecutionSequence`
        (:`then_0`
          ;[1 1 1] Teleport enemy to the endless void called death
          (`self.K2_SetActorLocation` self (0.0 0.0 0.0) false true))
        (:`then_1`
          (`AudioComponent.Stop` _fsproximityaudio)
          (`KismetSystemLibrary.Delay` 1.0)
          (`ActorComponent.Activate` _fsproximityaudio false))))))

(event `self.PawnSensing.OnSeePawn`
  (params (Pawn :type "Pawn Object Reference"))
  ;[1 1 1] Chase code with roar
  (bind _asplayer (cast `/Game/Player_Content/Player` Pawn))
  (`|ExecutionSequence`
    (:`then_0`
      (set `self.CanSeeEnemy?` true)
      (set `self.IsChasing?` true)
      (`|AIMoveTo` self (0.0 0.0 0.0) _asplayer
        (:`then`
          (`/Engine/EditorBlueprintResources/StandardMacros.DoOnce` false
            (:`Completed`
              (`AudioComponent.Play` (`self.Audio`) 0.0))))))
    (:`then_1`
      (`KismetSystemLibrary.RetriggerableDelay` 0.6)
      (set `self.CanSeeEnemy?` false))
    (:`then_2`
      (set `CharacterMovementComponent.MaxWalkSpeed` (`self.ChaseSpeed`) (`self.CharacterMovement`)))))

(event `Patrol`
  ;[1 1 1] Patrol
  (if (`self.Patrol Location 1`)
    (`self.Patrol locations` true
      (:`Out`
        (`|AIMoveTo` self (`self.Location 1`) null
          (:`OnSuccess`
            (`SceneComponent.K2_AddLocalRotation` (`self.Mesh`) (struct :`Yaw` -90.0) false false)
            (`self.Patrol locations` false true :!label _label_2
              (:`Out`
                (`|AIMoveTo` self (`self.Location 2`) null
                  (:`OnSuccess`
                    (`SceneComponent.K2_AddLocalRotation` (`self.Mesh`) (struct :`Yaw` -90.0) false false)
                    (`self.Patrol locations` false false true :!label _label_3
                      (:`Out`
                        (`|AIMoveTo` self (`self.Location 3`) null
                          (:`OnSuccess`
                            (`self.Patrol locations` false false false true :!label _label_4
                              (:`Out`
                                (`|AIMoveTo` self (`self.Location 4`) null
                                  (:`OnSuccess`
                                    (`SceneComponent.K2_AddLocalRotation` (`self.Mesh`) (struct :`Yaw` -90.0) false false)
                                    (`self.Patrol locations` false false false false true :!label _label_5
                                      (:`Out`
                                        (`|AIMoveTo` self (`self.Location 5`) null
                                          (:`OnSuccess`
                                            (`SceneComponent.K2_AddLocalRotation` (`self.Mesh`) (struct :`Yaw` -90.0) false false)
                                            (`self.Patrol locations` false false false false false true :!label _label_6
                                              (:`Out`
                                                (`|AIMoveTo` self (`self.Location 6`) null
                                                  (:`OnSuccess`
                                                    (`SceneComponent.K2_AddLocalRotation` (`self.Mesh`) (struct :`Yaw` -90.0) false false)
                                                    (`self.Patrol locations` false false true
                                                      (:`Out`
                                                        (`|AIMoveTo` self (`self.Location 3`) null
                                                          (:`OnSuccess`
                                                            (`SceneComponent.K2_AddLocalRotation` (`self.Mesh`) (struct :`Yaw` -90.0) false false)
                                                            (`self.Patrol locations` false true
                                                              (:`Out`
                                                                (`|AIMoveTo` self (`self.Location 2`) null
                                                                  (:`OnSuccess`
                                                                    (`SceneComponent.K2_AddLocalRotation` (`self.Mesh`) (struct :`Yaw` 180.0) false false)
                                                                    (`self.Patrol locations` true
                                                                      (:`Out`
                                                                        (`|AIMoveTo` self (`self.Location 1`) null
                                                                          (:`then`
                                                                            (`self.K2_DestroyActor`)))))))))))))))))))))))))))))))))))))
    (elif (`self.Patrol Location 2`)
      (goto _label_2)
      (elif (`self.Patrol Location 3`)
        (goto _label_3)
        (elif (`self.Patrol Location 4`)
          (goto _label_4)
          (elif (`self.Patrol Location 5`)
            (goto _label_5)
            (elif (`self.Patrol Location 6`)
              (goto _label_6))))))))

(fn `UserConstructionScript`)