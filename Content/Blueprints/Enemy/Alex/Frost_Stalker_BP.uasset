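; Frost Stalker enemy that hurts the player on contact and plays positional bone-crack and call-out response sounds.
; Hitting shovel snow freezes it by setting its capsule Static until the snow's StopMoving flag clears.
; A DoOnce-gated hurt overlap deducts lives from the game instance, triggers the player's hurt animation or death call, then teleports the stalker to world origin.
; The Response event also ends the player's call-out.
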(event `self.ReceiveHit`
  (params (MyComp :type "PrimitiveComponent Object Reference") (Other :type "Actor Object Reference") (OtherComp :type "PrimitiveComponent Object Reference") (bSelfMoved :type Boolean) (HitLocation :type "Vector Structure") (HitNormal :type "Vector Structure") (NormalImpulse :type "Vector Structure") (Hit :type "HitResult Structure (by ref)"))
  (bind _capsulecomponent (`self.CapsuleComponent`))
  ;[1 1 1] Destroy snow mechanic
  (bind _asshovel_snow_bp (cast `/Game/Snow/SnowShovel/ShovelSnow_BP` Other))
  (`SceneComponent.SetMobility` _capsulecomponent "Static")
  (`KismetSystemLibrary.Delay` 3.0)
  (if (`/Game/Snow/SnowShovel/ShovelSnow_BP.StopMoving` _asshovel_snow_bp) :!label _label
    (`KismetSystemLibrary.Delay` 2.0)
    (goto _label)
    (else
      (`SceneComponent.SetMobility` _capsulecomponent "Movable"))))

(event `Response'`
  ;[1 1 1] Call Out Respond
  (`GameplayStatics.PlaySoundAtLocation` "/Game/Audio/FrostStalkerSounds/FrostResponse.FrostResponse" (`SceneComponent.K2_GetComponentLocation` (`self.Mesh`)) (struct) 1.0 1.0 0.0 "/Game/Blueprints/PlayerAttenuation.PlayerAttenuation" null null)
  (bind _outactors (`GameplayStatics.GetAllActorsOfClass` "/Game/Player_Content/Player.Player_C"))
  (`/Game/Player_Content/Player.End Call Out` _outactors))

(event `self.ReceiveTick`
  (params (DeltaSeconds :type "Float (single-precision)"))
  ;[1 1 1] Constant Bone Crack sound
  (`KismetSystemLibrary.Delay` 3.0)
  (`GameplayStatics.PlaySoundAtLocation` "/Game/Audio/FrostStalkerSounds/SFX_BoneBreaking.SFX_BoneBreaking" (`SceneComponent.K2_GetComponentLocation` (`self.Mesh`)) (struct) 1.0 1.0 0.0 "/Game/Blueprints/PlayerAttenuation.PlayerAttenuation" null null))

(event `self.ReceiveBeginPlay`
  (set `self.Starting Location` (`self.K2_GetActorLocation`)))

(event `self.HurtCollision.OnComponentBeginOverlap`
  (params (OverlappedComponent :type "PrimitiveComponent Object Reference") (OtherActor :type "Actor Object Reference") (OtherComp :type "PrimitiveComponent Object Reference") (OtherBodyIndex :type Integer) (bFromSweep :type Boolean) (SweepResult :type "HitResult Structure (by ref)"))
  ;[1 1 1] If enemy collides with player, lose 1 life and player can't move for 2 seconds (enough time for animation to play)
  (bind _asplayer (cast `/Game/Player_Content/Player` OtherActor))
  (bind _asfrostbitten_game_inst_bp (cast `/Game/Blueprints/FrostbittenGameInst_BP` (`GameplayStatics.GetGameInstance`)))
  (`/Engine/EditorBlueprintResources/StandardMacros.DoOnce` false :!label _label_2
    (:`Completed`
      (bind _output_get (set `/Game/Blueprints/FrostbittenGameInst_BP.Lives` (- (`/Game/Blueprints/FrostbittenGameInst_BP.Lives` _asfrostbitten_game_inst_bp) 2) _asfrostbitten_game_inst_bp))
      (`|ExecutionSequence`
        (:`then_0`
          (if (> _output_get 0)
            (`/Game/Player_Content/Player.HurtPlayerAnimation` _asplayer)
            (`GameplayStatics.PlaySound2D` "/Game/Audio/FrostStalkerSounds/SFX_FrostRoar_main.SFX_FrostRoar_main" 1.0 1.0 0.0 null null)
            (else
              (`/Game/Blueprints/FrostbittenGameInst_BP.PlayerDiedFrost` _asfrostbitten_game_inst_bp)))
          (`KismetSystemLibrary.Delay` 0.1)
          ;[1 1 1] Teleport enemy to the endless void called death
          (`self.K2_SetActorLocation` self (0.0 0.0 0.0) false true)
          (goto _label_2 :!via `Reset`))
        (:`then_1`
          (if (<= _output_get 0)
            (`GameplayStatics.PlaySound2D` "/Game/Audio/FrostStalkerSounds/SFX_FrostRoar_main.SFX_FrostRoar_main" 1.0 1.0 0.0 null null)
            (`self.K2_SetActorLocation` self (0.0 0.0 0.0) false true)
            (goto _label_2 :!via `Reset`)))))))

(fn `UserConstructionScript`)