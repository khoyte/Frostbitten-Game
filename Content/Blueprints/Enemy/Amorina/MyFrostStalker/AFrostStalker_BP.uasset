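; Frost Stalker enemy character that hurts the player on overlap and makes bone-crack, roar and call-out response sounds.
; A hit deducts game-instance lives, triggers hurt or death handling, then teleports the stalker to its start and sets the AI blackboard's Teleported flag.
; Shoveled snow immobilizes it by switching capsule mobility.
; Tick sets FSInView from a padded screen-bounds test, while exposed events switch walk/run speed and anim classes or pause animation.
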(event `self.ReceiveHit`
  (params (MyComp :type "PrimitiveComponent Object Reference") (Other :type "Actor Object Reference") (OtherComp :type "PrimitiveComponent Object Reference") (bSelfMoved :type Boolean) (HitLocation :type "Vector Structure") (HitNormal :type "Vector Structure") (NormalImpulse :type "Vector Structure") (Hit :type "HitResult Structure (by ref)"))
  (bind _capsulecomponent (`self.CapsuleComponent`))
  ;[1 1 1] Destroy snow mechanic
  (bind _asshovel_snow_bp (cast `/Game/Snow/SnowShovel/ShovelSnow_BP` Other))
  (`SceneComponent.SetMobility` _capsulecomponent "Static")
  (`KismetSystemLibrary.Delay` 3.0)
  (if (`/Game/Snow/SnowShovel/ShovelSnow_BP.StopMoving` _asshovel_snow_bp) :!label _label
    (`KismetSystemLibrary.Delay` 2.0)
    (goto _label)
    (else
      (`SceneComponent.SetMobility` _capsulecomponent "Movable"))))

(event `self.ReceiveBeginPlay`
  (set `self.StartingLocation` (`self.K2_GetActorLocation`)))

(event `Response'`
  ;[1 1 1] Call Out Respond
  (`GameplayStatics.PlaySoundAtLocation` "/Game/Audio/FrostStalkerSounds/Dial_FrostResponse_Alt.Dial_FrostResponse_Alt" (`SceneComponent.K2_GetComponentLocation` (`self.Mesh`)) (struct) 1.0 1.0 0.0 "/Game/Blueprints/PlayerAttenuation.PlayerAttenuation" null null)
  (bind _outactors (`GameplayStatics.GetAllActorsOfClass` "/Game/Player_Content/Player.Player_C"))
  (`/Game/Player_Content/Player.End Call Out` _outactors))

(event `self.ReceiveTick`
  (params (DeltaSeconds :type "Float (single-precision)"))
  (bind (_returnvalue_x _returnvalue_y) (`KismetMathLibrary.BreakVector2D` (`WidgetLayoutLibrary.GetViewportSize`)))
  (bind _screenlocation (`PlayerController.ProjectWorldLocationToScreen` (`GameplayStatics.GetPlayerController` 0) (`self.K2_GetActorLocation`) false))
  ;[1 1 1] Constant Bone Crack sound
  (`|ExecutionSequence`
    (:`then_0`
      (`KismetSystemLibrary.Delay` 3.0)
      (`GameplayStatics.PlaySoundAtLocation` "/Game/Audio/FrostStalkerSounds/SFX_BoneBreaking.SFX_BoneBreaking" (`SceneComponent.K2_GetComponentLocation` (`self.Mesh`)) (struct) 1.0 1.0 0.0 "/Game/Blueprints/PlayerAttenuation.PlayerAttenuation" null null))
    (:`then_1`
      (if (and (> (`KismetMathLibrary.BreakVector2D` _screenlocation) -600.0) (> (`.Y` (`KismetMathLibrary.BreakVector2D` _screenlocation)) -600.0) (< (`KismetMathLibrary.BreakVector2D` _screenlocation) (+ _returnvalue_x 600.0)) (< (`.Y` (`KismetMathLibrary.BreakVector2D` _screenlocation)) (+ _returnvalue_y 600.0)))
        (set `self.FSInView?` true)
        (else
          (set `self.FSInView?` false))))))

(event `StopCycleAnimation`
  ;[1 1 1] Events for poses
  (set `SkeletalMeshComponent.bPauseAnims` true (`self.Mesh`)))

(event `PlayCycleAnimation`
  ;[1 1 1] Events for poses
  (set `SkeletalMeshComponent.bPauseAnims` false (`self.Mesh`)))

(event `SetWalkingAnimationBP`
  ;[1 1 1] Events for poses
  (`SkeletalMeshComponent.SetAnimInstanceClass` (`self.Mesh`) "/Game/Blueprints/Enemy/Amorina/MyFrostStalker/AFrostStalker_AnimBP.AFrostStalker_AnimBP_C"))

(event `SetCycleAnimationBP`
  ;[1 1 1] Events for poses
  (`SkeletalMeshComponent.SetAnimInstanceClass` (`self.Mesh`) "/Game/Blueprints/Animation/NewFrostStalker_AnimBP.NewFrostStalker_AnimBP_C"))

(event `Walk`
  ;[1 1 1] Movement
  (set `CharacterMovementComponent.MaxWalkSpeed` 500.0 (`self.CharacterMovement`)))

(event `Run`
  ;[1 1 1] Movement
  (set `CharacterMovementComponent.MaxWalkSpeed` 750.0 (`self.CharacterMovement`)))

(event `self.HurtCollision.OnComponentBeginOverlap`
  (params (OverlappedComponent :type "PrimitiveComponent Object Reference") (OtherActor :type "Actor Object Reference") (OtherComp :type "PrimitiveComponent Object Reference") (OtherBodyIndex :type Integer) (bFromSweep :type Boolean) (SweepResult :type "HitResult Structure (by ref)"))
  (bind _sfx_froststalkerproximity_shorter (`self.SFX_FrostStalkerProximity_Shorter`))
  (bind _startinglocation (`self.StartingLocation`))
  ;[1 1 1] Hurt Collision
  (`/Engine/EditorBlueprintResources/StandardMacros.DoOnce` false :!label _label_2
    (:`Completed`
      (bind _asplayer (cast `/Game/Player_Content/Player` OtherActor)
        (:`then`
          (bind _asfrostbitten_game_inst_bp (cast `/Game/Blueprints/FrostbittenGameInst_BP` (`GameplayStatics.GetGameInstance`)))
          (`|ExecutionSequence`
            (:`then_0`
              (bind _output_get (set `/Game/Blueprints/FrostbittenGameInst_BP.Lives` (- (`/Game/Blueprints/FrostbittenGameInst_BP.Lives` _asfrostbitten_game_inst_bp) (`self.DamageDelt`)) _asfrostbitten_game_inst_bp))
              (if (> _output_get 0)
                (`/Game/Player_Content/Player.HurtPlayerAnimation` _asplayer)
                (`GameplayStatics.PlaySound2D` "/Game/Audio/FrostStalkerSounds/SFX_FrostRoar_main.SFX_FrostRoar_main" 1.0 1.0 0.0 null null)
                (else
                  (bind _returnvalue (`GameplayStatics.GetCurrentLevelName` true))
                  (if (`KismetStringLibrary.EqualEqual_StrStr` _returnvalue "Chapter3")
                    (`/Game/Blueprints/FrostbittenGameInst_BP.PlayerDiedTree` _asfrostbitten_game_inst_bp)
                    (else
                      (`/Game/Blueprints/FrostbittenGameInst_BP.PlayerDiedFrost` _asfrostbitten_game_inst_bp)))))
              (`KismetSystemLibrary.Delay` 0.1)
              (`self.K2_SetActorLocation` _startinglocation false true)
              (`|ExecutionSequence`
                (:`then_0`
                  (`GameplayStatics.PlaySoundAtLocation` "/Game/Audio/FrostStalkerSounds/FrostRoar.FrostRoar" _startinglocation (struct) 1.0 1.0 0.0 "/Game/Blueprints/PlayerAttenuation.PlayerAttenuation" null null))
                (:`then_1`
                  (`BlackboardComponent.SetValueAsBool` (`AIBlueprintHelperLibrary.GetBlackboard` (`AIBlueprintHelperLibrary.GetAIController` (`ActorComponent.GetOwner` (`self.Mesh`)))) "Teleported" true)
                  (goto _label_2 :!via `Reset`))))
            (:`then_1`
              (`AudioComponent.Stop` _sfx_froststalkerproximity_shorter)
              (`KismetSystemLibrary.Delay` 1.0)
              (`ActorComponent.Activate` _sfx_froststalkerproximity_shorter false))))
        (:`CastFailed`
          (goto _label_2 :!via `Reset`))))))

(fn `UserConstructionScript`)