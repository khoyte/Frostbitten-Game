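; Amorina mini-monster enemy that costs the player a life on contact, then screams and destroys itself.
; Lives live in the game instance, which triggers player death at zero; Walk and Run events set movement speed.
; Damage drains health, briefly applies burn speed and a burning flag that Tick polls for audio, and starts a delayed full-health regen.
; At zero health, a timeline animates a material parameter before destroying the actor.
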(event `self.ReceiveTick`
  (params (DeltaSeconds :type "Float (single-precision)"))
  (bind _burningaudio (`self.BurningAudio`))
  ;[1 1 1] SFX
  (`KismetSystemLibrary.Delay` 0.2)
  (`|ExecutionSequence`
    (:`then_1`
      (if (`self.IsBurning?`)
        (`/Engine/EditorBlueprintResources/StandardMacros.DoOnce` false :!label _label
          (:`Completed`
            (`ActorComponent.Activate` _burningaudio false)
            (goto _label :!via `Reset`)))
        (else
          (`AudioComponent.Stop` _burningaudio))))))

(event `Walk`
  ;[1 1 1] Set walk and run speeds of actual mini-monster
  (set `CharacterMovementComponent.MaxWalkSpeed` 150.0 (`self.CharacterMovement`)))

(event `Run`
  ;[1 1 1] Set walk and run speeds of actual mini-monster
  (set `CharacterMovementComponent.MaxWalkSpeed` 300.0 (`self.CharacterMovement`)))

(event `self.ReceiveHit`
  (params (MyComp :type "PrimitiveComponent Object Reference") (Other :type "Actor Object Reference") (OtherComp :type "PrimitiveComponent Object Reference") (bSelfMoved :type Boolean) (HitLocation :type "Vector Structure") (HitNormal :type "Vector Structure") (NormalImpulse :type "Vector Structure") (Hit :type "HitResult Structure (by ref)"))
  ;[1 1 1] tonnie kill monster
  (cast `/Game/Player_Content/Player` Other)
  (`/Engine/EditorBlueprintResources/StandardMacros.DoOnce` false :!label _label_2
    (:`Completed`
      (bind _asfrostbitten_game_inst_bp (cast `/Game/Blueprints/FrostbittenGameInst_BP` (`GameplayStatics.GetGameInstance`)))
      (bind _lives (`/Game/Blueprints/FrostbittenGameInst_BP.Lives` _asfrostbitten_game_inst_bp))
      (set `/Game/Blueprints/FrostbittenGameInst_BP.Lives` (- _lives 1) _asfrostbitten_game_inst_bp)
      (if (<= _lives 0)
        (`/Game/Blueprints/FrostbittenGameInst_BP.PlayerDiedTree` _asfrostbitten_game_inst_bp))
      (`GameplayStatics.PlaySound2D` "/Game/Audio/SFX/SFX_Scream1.SFX_Scream1" 0.3 1.0 0.0 null null)
      (`self.K2_DestroyActor`)
      (`KismetSystemLibrary.Delay` 0.2)
      (goto _label_2 :!via `Reset`))))

(event `self.ReceiveAnyDamage`
  (params (Damage :type "Float (single-precision)") (DamageType :type "DamageType Object Reference") (InstigatedBy :type "Controller Object Reference") (DamageCauser :type "Actor Object Reference"))
  ;[1 1 1] Raytrace hit effect, lose hp, get slowed
  (`|ExecutionSequence`
    (:`then_0`
      (bind _output_get (set `self.EnemyHealth` (- (`self.EnemyHealth`) Damage)))
      (if (<= _output_get 0.0)
        (bind (_direction _fire) (`Timeline|FIreDie`)
          (:`Update`
            (`MeshComponent.SetScalarParameterValueOnMaterials` (`self.Mesh`) "Apperance" _fire))
          (:`Finished`
            (`AudioComponent.Stop` (`self.ProximityAudio`))
            (`AudioComponent.Stop` (`self.BurningAudio`))
            (`self.K2_DestroyActor`)))))
    (:`then_1`
      (set `CharacterMovementComponent.MaxWalkSpeed` (`self.Burning Walk Speed`) (`self.CharacterMovement`))
      (set `self.IsBurning?` true)
      (`KismetSystemLibrary.Delay` 1.0)
      (set `CharacterMovementComponent.MaxWalkSpeed` (`self.Run Speed`) (`self.CharacterMovement`))
      (set `self.IsBurning?` false))
    (:`then_2`
      ;;[1 1 1] After 5 seconds of getting hit, monster will regen to full hp, punishes player for taking too long
      (`KismetSystemLibrary.Delay` 5.0)
      (set `self.EnemyHealth` (`self.Max Enemy Health`)))))

(fn `UserConstructionScript`)