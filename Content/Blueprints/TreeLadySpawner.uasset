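; Tree Lady spawner that spawns enemies, noted as the frost stalker, when the Player leaves its overlap.
; It sets the "Teleported" blackboard flag, then searches SpawnTarget actors for the one nearest its collision component.
; It issues two offset spawns around that point, one being MiniMonster_BP, then waits out a cooldown before re-arming.
; RespawnEnemy is empty, and a TargetPoint-based teleport toward the Player is left disconnected.
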(event `self.ReceiveActorEndOverlap`
  (params (OtherActor :type "Actor Object Reference"))
  (bind _new (`self.New`))
  (bind _target (`self.Target`))
  (bind _new_2 (`self.New`))
  (bind _returnvalue (`SceneComponent.K2_GetComponentLocation` (`self.CollisionComponent`)))
  ;[1 1 1] Spawn the frost stalker
  (if (not (`self.Stop`))
    (cast `/Game/Player_Content/Player` OtherActor)
    (`BlackboardComponent.SetValueAsBool` (`AIBlueprintHelperLibrary.GetBlackboard` (`AIBlueprintHelperLibrary.GetAIController` null)) "Teleported" true)
    (set `self.Stop` true)
    (bind _outactors (`GameplayStatics.GetAllActorsOfClass` "/Game/Blueprints/SpawnTarget.SpawnTarget_C"))
    ;[1 1 1] Get and set Target Spawn location
    (for _array_element _outactors
      (`|ExecutionSequence`
        (:`then_0`
          (`/Engine/EditorBlueprintResources/StandardMacros.DoOnce` false :!label _label
            (:`Completed`
              (bind _returnvalue_2 (`SceneComponent.K2_GetComponentLocation` (`/Game/Blueprints/SpawnTarget.DefaultSceneRoot` _array_element)))
              (set `self.TargetSpawn` _returnvalue_2))))
        (:`then_1`
          (set `self.Target` (`KismetMathLibrary.VSize` (- (`self.TargetSpawn`) _returnvalue)))
          (set `self.New` (`KismetMathLibrary.VSize` (- _returnvalue_2 _returnvalue)))
          (if (< _new 0.0)
            (set `self.New` (* _new -1.0)))
          (if (< _target 0.0)
            (set `self.Target` (* _target -1.0)))
          (if (> (`self.Target`) _new_2)
            (set `self.Target` _new_2)
            (bind _output_get (set `self.TargetSpawn` _returnvalue_2))
            (set `self.TargetSpawn_0` (+ _output_get (30.0 50.0 0.0)))
            (set `self.TargetSpawn_1` (+ _output_get (-30.0 -50.0 0.0)))))))
    (`|SpawnActorFromClass` "/Game/Blueprints/Enemy/Amorina/MiniMonsters/MiniMonster_BP.MiniMonster_BP_C" (`KismetMathLibrary.Conv_VectorToTransform` (`self.TargetSpawn_0`)) "Undefined" "OverrideRootScale" null null)
    (`self.K2_AddActorWorldRotation` (struct :`Yaw` 180.0))
    (`|SpawnActorFromClass` "/Game/Blueprints/Enemy/Amorina/MiniMonsters/MiniMonster_BP.MiniMonster_BP_C" (`KismetMathLibrary.Conv_VectorToTransform` (`self.TargetSpawn_1`)) "Undefined" "OverrideRootScale" null null)
    (`self.K2_AddActorWorldRotation` (struct :`Yaw` 180.0))
    (`KismetSystemLibrary.Delay` 15.0)
    (set `self.Stop` false)
    (goto _label :!via `Reset`)))

(event `RespawnEnemy`)

(fn `UserConstructionScript`)