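; Blink component that drains eye hydration over time, forces a blink when it runs out, and tracks whether its owner can see.
; A looping one-second timer drains hydration, with an added delay when it is full, and triggers Blinks at zero.
; Blinks spawns a blink widget behind a DoOnce, which EndBlink resets while refilling hydration.
; Tick clears CanSee while blinking or in darkness without a flashlight.
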(event `self.ReceiveBeginPlay`
  (`KismetSystemLibrary.K2_SetTimerDelegate` (delegate `Hydration Loop`) 1.0 true)
  (bind _returnvalue (`|CreateWidget` "/Game/Blueprints/Widgets/HUD_BP.HUD_BP_C"))
  (set `self.HUD_BP` _returnvalue)
  (set `/Game/Blueprints/Widgets/HUD_BP.BlinkComponent` self _returnvalue)
  (`UserWidget.AddToPlayerScreen` _returnvalue 0))

(event `Hydration Loop`
  ;[1 1 1] Eye Hydration level drain loop
  (set `self.CanBlink` true)
  (if (== (`self.EyeHydrationMax`) (`self.EyeHydration`))
    (`KismetSystemLibrary.Delay` (`self.HydrationDelay`) :!label _label)
    (else
      (`|ExecutionSequence`
        (:`then_0`
          (`/Engine/EditorBlueprintResources/StandardMacros.DoOnce` false :!enabledstate Disabled :!via `Reset`
            (:`Completed`
              (goto _label))))
        (:`then_1`
          _))))
  (bind _output_get (set `self.EyeHydration` (- (`self.EyeHydration`) (`self.HydrationDrain`))))
  (if (<= _output_get 0.0)
    (`self.Blinks`)))

(event `Blinks`
  ;[1 1 1] Blinking
  (set `self.CanBlink` false)
  (`/Engine/EditorBlueprintResources/StandardMacros.DoOnce` false :!label _label_2
    (:`Completed`
      (set `self.Blinking` true)
      (bind _returnvalue (`|CreateWidget` "/Game/Blueprints/Widgets/BlinkHUD_BP.BlinkHUD_BP_C"))
      (set `self.BlinkHUD_BP` _returnvalue)
      (set `/Game/Blueprints/Widgets/BlinkHUD_BP.BlinkComponent` self _returnvalue)
      (`UserWidget.AddToPlayerScreen` _returnvalue 0))))

(event `End Blink`
  ;[1 1 1] Blinking
  (set `self.Blinking` false)
  (set `self.EyeHydration` (`self.EyeHydrationMax`))
  (goto _label_2 :!via `Reset`))

(event `self.ReceiveTick`
  (params (DeltaSeconds :type "Float (single-precision)"))
  ;[1 1 1] Set can see
  (set `self.CanSee` (not (or (and (`self.Dark`) (not (`self.Flashlight`))) (`self.Blinking`)))))